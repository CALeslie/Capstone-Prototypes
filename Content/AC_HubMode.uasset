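; AC_HubMode is a hub-mode component that places players and gathers state for the hub level.
; SetUpPlayers shuffles the BP_PlayerStart actors, teleports each game mode player to one with a small height offset, then shows them and refreshes their camera reference.
; HubSetup caches hub doors and spotlight controls and records last-place players, including ties, treating the highest score as last place.
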(event EventBeginPlay)

(event EventTick
  (params (DeltaSeconds :type Float%20%28single-precision%29)))

(fn SetUpPlayers
  (bind _outactors (Actor|GetAllActorsOfClass "/Game/Minigame/Blueprints/BP_PlayerStart.BP_PlayerStart_C"))
  (bind _output_get (LocalVariables|SetPlayerStarts _outactors))
  (Utilities|Array|Shuffle _output_get)
  (for (_array_element _array_index) (LocalVariables|GetPlayerStarts)
    (Transformation|SetActorLocationAndRotation (Utilities|Array|Get(acopy) (Variables|/Game/Minigame/Blueprints/BP_MinigameMode.BP_MinigameMode_C|GetPlayers (Variables|Default|GetGameModeRef)) _array_index) (Math|Vector|MakeVector (.x (Transformation|GetActorLocation _array_element)) (.y (Transformation|GetActorLocation _array_element)) (+ (.z (Transformation|GetActorLocation _array_element)) 30.62)) (Transformation|GetActorRotation _array_element) false true)
    (Default|TogglePlayerVisibility (Utilities|Array|Get(acopy) (Variables|/Game/Minigame/Blueprints/BP_MinigameMode.BP_MinigameMode_C|GetPlayers (Variables|Default|GetGameModeRef)) _array_index) true)
    (Default|RefreshCameraRef (Utilities|Array|Get(acopy) (Variables|/Game/Minigame/Blueprints/BP_MinigameMode.BP_MinigameMode_C|GetPlayers (Variables|Default|GetGameModeRef)) _array_index))))

(fn HubSetup
  (params (GameModeRef :type BP%20Minigame%20Mode%20Object%20Reference))
  (Utilities|IsValid (Variables|Default|GetGameModeRef)
    (:Is%20Valid
      _)
    (:Is%20Not%20Valid
      (Variables|Default|SetGameModeRef GameModeRef)))
  (CallFunction|SetLastPlacePlayers)
  (bind _outactors (Actor|GetAllActorsOfClass "/Game/Minigame/Blueprints/Minigames/Hub/BP_HubDoor.BP_HubDoor_C"))
  (Variables|Default|SetHubDoors _outactors)
  (bind _outactors_2 (Actor|GetAllActorsOfClass "/Game/Minigame/Blueprints/BP_SpotLightControl.BP_SpotLightControl_C"))
  (Variables|Default|SetHubDoorLights _outactors_2))

(fn SetLastPlacePlayers
  (bind _lastplaceplayers (Variables|Default|GetLastPlacePlayers))
  (for (_array_element _array_index) (Variables|/Game/Minigame/Blueprints/BP_MinigameMode.BP_MinigameMode_C|GetPlayerScores (Variables|Default|GetGameModeRef))
    (if (> _array_element (LocalVariables|GetLastPlaceScore))
      (LocalVariables|SetLastPlaceScore _array_element)
      (Utilities|Array|Clear _lastplaceplayers)
      (Utilities|Array|AppendArray _lastplaceplayers (Utilities|Array|MakeArray (Utilities|Array|Get(acopy) (Variables|/Game/Minigame/Blueprints/BP_MinigameMode.BP_MinigameMode_C|GetPlayers (Variables|Default|GetGameModeRef)) _array_index)))
      (elif (== _array_element (LocalVariables|GetLastPlaceScore))
        (Utilities|Array|AppendArray (Variables|Default|GetLastPlacePlayers) (Utilities|Array|MakeArray (Utilities|Array|Get(acopy) (Variables|/Game/Minigame/Blueprints/BP_MinigameMode.BP_MinigameMode_C|GetPlayers (Variables|Default|GetGameModeRef)) _array_index)))))))