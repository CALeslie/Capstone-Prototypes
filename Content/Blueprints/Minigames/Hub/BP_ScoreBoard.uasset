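; BP_ScoreBoard is a minigame hub scoreboard actor that displays point totals for up to four players.
; SetPlayerScore switches on a player index and writes the score, with a "points" suffix, to that player's text element.
; The event graph and construction script are empty, so the board changes only when SetPlayerScore is called.
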(event EventBeginPlay)

(event Collision|EventActorBeginOverlap
  (params (OtherActor :type Actor%20Object%20Reference)))

(event EventTick
  (params (DeltaSeconds :type Float%20%28single-precision%29)))

(fn ConstructionScript)

(fn SetPlayerScore
  (params (Index :type Integer) (Score :type Integer))
  (bind _returnvalue (Utilities|String|ToString(Integer) Score))
  (bind _returnvalue_2 (Utilities|String|Append _returnvalue " points"))
  (bind _returnvalue_3 (Utilities|Text|ToText(String) _returnvalue_2))
  (switch int Index
    (:0
      (Rendering|Components|TextRender|SetText (Variables|Default|GetP1PointsText) _returnvalue_3))
    (:1
      (Rendering|Components|TextRender|SetText (Variables|Default|GetP2PointsText) _returnvalue_3))
    (:2
      (Rendering|Components|TextRender|SetText (Variables|Default|GetP3PointsText) _returnvalue_3))
    (:3
      (Rendering|Components|TextRender|SetText (Variables|Default|GetP4PointsText) _returnvalue_3))))