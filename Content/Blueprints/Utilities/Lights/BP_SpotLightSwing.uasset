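; BP_SpotLightSwing is a light utility Blueprint that swings and slowly turns its Pivot component, by its name for a swinging spotlight.
; The LightSwing timeline starts on BeginPlay and drives Pivot's roll and pitch, adding a fixed yaw step each update, so turn speed depends on frame rate.
; Tick counts SwingTimer up or down based on Back, but this graph neither reads the timer nor sets the flag.
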(event EventBeginPlay
  (bind _pivot (Variables|Default|GetPivot))
  (|CallParentFunction)
  (bind (_direction _rotation_x _rotation_y) (Timeline|LightSwing Play)
    (:Update
      (Transformation|SetRelativeRotation _pivot (Math|Rotator|MakeRotator _rotation_x _rotation_y (.yaw (Variables|/Script/Engine.SceneComponent|GetRelativeRotation _pivot))) false false)
      (Transformation|AddRelativeRotation _pivot (Math|Rotator|MakeRotator 0.0 0.0 0.3) false false))))

(event Collision|EventActorBeginOverlap
  (params (OtherActor :type Actor%20Object%20Reference)))

(event EventTick
  (params (DeltaSeconds :type Float%20%28single-precision%29))
  (if (Variables|Default|GetBack)
    (Variables|Default|SetSwingTimer (- (Variables|Default|GetSwingTimer) DeltaSeconds))
    (else
      (Variables|Default|SetSwingTimer (+ (Variables|Default|GetSwingTimer) DeltaSeconds)))))

(fn ConstructionScript
  (|CallParentFunction))