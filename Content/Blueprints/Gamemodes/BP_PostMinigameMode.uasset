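; Game mode for the post-minigame screen, showing four players' previous totals and points earned, then moving on to the next level.
; On BeginPlay it reads last minigame ranks from BP_GameInstance, fills the score widget, then adds rank-based points to stored scores, with higher rank numbers earning more.
; Chained timelines fade the screen in and, after a pause, out.
; It then increments the round and opens either the hub or post-game level.
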(event EventBeginPlay
  (|CallParentFunction)
  (bind _asbp_game_instance (Utilities|Casting|CastToBP_GameInstance (Game|GetGameInstance)))
  (Variables|Default|SetGameInstance _asbp_game_instance)
  (CallFunction|SetupPostMinigame)
  (CallFunction|DisplayNewScores (Variables|/Game/Blueprints/Utilities/BP_GameInstance.BP_GameInstance_C|GetPrevMinigameRanks (Variables|Default|GetGameInstance)))
  (CallFunction|AwardPoints (Variables|/Game/Blueprints/Utilities/BP_GameInstance.BP_GameInstance_C|GetPrevMinigameRanks (Variables|Default|GetGameInstance)))
  (bind _opacity (Timeline|FadeInPostMinigame_ PlayFromStart)
    (:Update
      (CallFunction|SetFadeOpacity _opacity))
    (:Finished
      (bind _opacity_2 (Timeline|FadeInScores_ PlayFromStart)
        (:Update
          (Variables|/Script/UMG.Widget|SetRenderOpacity (Variables|/Game/Blueprints/Widgets/WBP_PostMinigame.WBP_PostMinigame_C|GetPostMinigameCanvas (Variables|Default|GetPostMinigameUI)) _opacity_2))
        (:Finished
          (Utilities|FlowControl|Delay 5.0) ; Five second delay before transition
          (bind _opacity_3 (Timeline|FadeOutPostMinigame_ PlayFromStart)
            (:Update
              ;[1 1 1] Fades out score screen while fading in black fade
              (CallFunction|SetFadeOpacity _opacity_3)
              (bind _result (Math|Float|NegateFloat _opacity_3)
                (:%20%20
                  (Variables|/Script/UMG.Widget|SetRenderOpacity (Variables|/Game/Blueprints/Widgets/WBP_PostMinigame.WBP_PostMinigame_C|GetPostMinigameCanvas (Variables|Default|GetPostMinigameUI)) (+ _result 1.0)))))
            (:Finished
              ;[1 1 1] Increments current round number and checks for end of game
              (Math|Integer|IncrementInt (Variables|/Game/Blueprints/Utilities/BP_GameInstance.BP_GameInstance_C|GetCurrRound (Variables|Default|GetGameInstance))
                (:%20%20
                  (if (>= (Variables|/Game/Blueprints/Utilities/BP_GameInstance.BP_GameInstance_C|GetCurrRound (Variables|Default|GetGameInstance)) (Variables|/Game/Blueprints/Utilities/BP_GameInstance.BP_GameInstance_C|GetNumRounds (Variables|Default|GetGameInstance)))
                    (Game|OpenLevel(byObjectReference) "/Game/Environments/Levels/PostGameLevel.PostGameLevel")
                    (else
                      (Game|OpenLevel(byObjectReference) "/Game/Environments/Levels/HubLevel.HubLevel"))))))))))))

(event EventTick
  (params (DeltaSeconds :type Float%20%28single-precision%29))
  (|CallParentFunction DeltaSeconds) ; This node is disabled and will not be called.\nDrag off pins to build functionality.
)

(fn ConstructionScript
  (|CallParentFunction))

(fn DisplayNewScores
  (params (PrevGameRanks :type Array%20of%20Integers))
  (bind _postminigameui (Variables|Default|GetPostMinigameUI))
  (bind _postminigameui_2 (Variables|Default|GetPostMinigameUI))
  (for (_array_element _array_index) PrevGameRanks
    (bind _points (CallFunction|GetPointsfromRank _array_element))
    (switch int _array_index
      (:0
        (Rendering|Components|TextRender|SetText (Variables|/Game/Blueprints/Widgets/WBP_PostMinigame.WBP_PostMinigame_C|GetP1AddedScoreText _postminigameui) (Utilities|Text|ToText(String) (Utilities|String|Append "+" (Utilities|String|ToString(Integer) _points)))))
      (:1
        (Rendering|Components|TextRender|SetText (Variables|/Game/Blueprints/Widgets/WBP_PostMinigame.WBP_PostMinigame_C|GetP2AddedScoreText _postminigameui) (Utilities|Text|ToText(String) (Utilities|String|Append "+" (Utilities|String|ToString(Integer) _points)))))
      (:2
        (Rendering|Components|TextRender|SetText (Variables|/Game/Blueprints/Widgets/WBP_PostMinigame.WBP_PostMinigame_C|GetP3AddedScoreText _postminigameui) (Utilities|Text|ToText(String) (Utilities|String|Append "+" (Utilities|String|ToString(Integer) _points)))))
      (:3
        (Rendering|Components|TextRender|SetText (Variables|/Game/Blueprints/Widgets/WBP_PostMinigame.WBP_PostMinigame_C|GetP4AddedScoreText _postminigameui) (Utilities|Text|ToText(String) (Utilities|String|Append "+" (Utilities|String|ToString(Integer) _points)))))))
  (for _index (range 0 3)
    (switch int _index
      (:0
        (Rendering|Components|TextRender|SetText (Variables|/Game/Blueprints/Widgets/WBP_PostMinigame.WBP_PostMinigame_C|GetP1OldScoreText _postminigameui_2) (Utilities|Text|ToText(Integer) (Utilities|Array|Get(acopy) (Variables|/Game/Blueprints/Utilities/BP_GameInstance.BP_GameInstance_C|GetPlayerScores (Variables|Default|GetGameInstance)) _index))))
      (:1
        (Rendering|Components|TextRender|SetText (Variables|/Game/Blueprints/Widgets/WBP_PostMinigame.WBP_PostMinigame_C|GetP2OldScoreText _postminigameui_2) (Utilities|Text|ToText(Integer) (Utilities|Array|Get(acopy) (Variables|/Game/Blueprints/Utilities/BP_GameInstance.BP_GameInstance_C|GetPlayerScores (Variables|Default|GetGameInstance)) _index))))
      (:2
        (Rendering|Components|TextRender|SetText (Variables|/Game/Blueprints/Widgets/WBP_PostMinigame.WBP_PostMinigame_C|GetP3OldScoreText _postminigameui_2) (Utilities|Text|ToText(Integer) (Utilities|Array|Get(acopy) (Variables|/Game/Blueprints/Utilities/BP_GameInstance.BP_GameInstance_C|GetPlayerScores (Variables|Default|GetGameInstance)) _index))))
      (:3
        (Rendering|Components|TextRender|SetText (Variables|/Game/Blueprints/Widgets/WBP_PostMinigame.WBP_PostMinigame_C|GetP4OldScoreText _postminigameui_2) (Utilities|Text|ToText(Integer) (Utilities|Array|Get(acopy) (Variables|/Game/Blueprints/Utilities/BP_GameInstance.BP_GameInstance_C|GetPlayerScores (Variables|Default|GetGameInstance)) _index)))))))

(fn SetupPostMinigame
  (bind _returnvalue (UserInterface|CreateWidget "/Game/Blueprints/Widgets/WBP_PostMinigame.WBP_PostMinigame_C"))
  (bind _output_get (Variables|Default|SetPostMinigameUI _returnvalue))
  (UserInterface|Viewport|AddtoViewport _output_get 0)
  (CallFunction|CreateFadeWidget))

(fn GetPointsfromRank
  (params (Rank :type Integer))
  (switch int Rank
    (:1
      (return 0))
    (:2
      (return 2))
    (:3
      (return 3))
    (:4
      (return 5))))

(fn AwardPoints
  (params (MinigameRanks :type Array%20of%20Integers))
  (LocalVariables|SetPlayer%20Ranks MinigameRanks)
  (for (_array_element _array_index) (Variables|/Game/Blueprints/Utilities/BP_GameInstance.BP_GameInstance_C|GetPlayerScores (Variables|Default|GetGameInstance))
    (bind _points (CallFunction|GetPointsfromRank (Utilities|Array|Get(acopy) (LocalVariables|GetPlayer%20Ranks) _array_index)))
    (Utilities|Array|SetArrayElem (Variables|/Game/Blueprints/Utilities/BP_GameInstance.BP_GameInstance_C|GetPlayerScores (Variables|Default|GetGameInstance)) _array_index (+ _array_element _points))))