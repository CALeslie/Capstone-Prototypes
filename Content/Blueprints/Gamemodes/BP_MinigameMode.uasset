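; Game mode for four-player local minigames, providing shared setup and helper functions for players, UI and game state.
; SpawnPlayers recreates local controllers, possesses hidden, color-coded characters, then registers them with the dev menu and loads or creates saved settings.
; Helpers toggle player control and visibility and drive countdown, timer and fade widgets, with timer text refreshed once per second.
; Round, score and state changes are written to the game instance.
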(event EventBeginPlay
  (bind _returnvalue (UserInterface|CreateWidget "/Game/Blueprints/Widgets/WBP_DevMenu.WBP_DevMenu_C"))
  (bind _output_get (Variables|Default|SetDevMenuRef _returnvalue))
  (UserInterface|Viewport|AddtoViewport _output_get 0))

(event EventTick
  (params (DeltaSeconds :type Float%20%28single-precision%29)))

(event EventHandleStartingNewPlayer
  (params (NewPlayer :type Player%20Controller%20Object%20Reference)))

(event EventPostLogin
  (params (NewPlayer :type Player%20Controller%20Object%20Reference)))

(fn ConstructionScript)

(fn SpawnPlayers
  (bind _returnvalue (Game|GetPlayerController 0))
  (for _index (range 0 3)
    (Class|GameplayStatics|RemovePlayer (Class|GameplayStatics|GetPlayerControllerfromID _index) true))
  (Variables|Default|SetDefaultPawnClass "/Game/Blueprints/Characters/BP_MinigameCharacter.BP_MinigameCharacter_C")
  (for _index_2 (range 0 3)
    ;[1 1 1] Creates player controller, if valid spawns character pawn at player start entity and then possesses pawn with that controller
    (bind _returnvalue_2 (Class|GameplayStatics|CreatePlayer -1))
    (if (Utilities|IsValid _returnvalue_2)
      (bind _returnvalue_3 (Game|SpawnActorfromClass "/Game/Blueprints/Characters/BP_MinigameCharacter.BP_MinigameCharacter_C" (Math|Transform|MakeTransform "0, 0, 0" "0, 0, 0" "1.000000,1.000000,1.000000") "AlwaysSpawn" "MultiplyWithRoot" 0 0))
      (Pawn|Possess (Class|GameplayStatics|GetPlayerControllerfromID _index_2) _returnvalue_3)
      (Default|TogglePlayerVisibility _returnvalue_3 false)
      (Variables|/Game/Blueprints/Characters/BP_MinigameCharacter.BP_MinigameCharacter_C|SetPlayerID _returnvalue_3 _index_2)
      (Utilities|Array|AppendArray (Variables|Default|GetPlayers) (Utilities|Array|MakeArray _returnvalue_3))
      (Players|SetPlayerMaterial (Variables|/Script/Engine.Character|GetMesh _returnvalue_3) _index_2)))
  ;[1 1 1] Required to clean up default spawned controller
  (Class|GameModeBase|RestartPlayer _returnvalue)
  (bind _asbp_minigame_character (Utilities|Casting|CastToBP_MinigameCharacter (Pawn|GetControlledPawn _returnvalue)))
  (Default|TogglePlayerVisibility _asbp_minigame_character false)
  ;[1 1 1] Sends references of players back to movement controls UI to be modifiable on change
  (bind _foundwidgets (Widget|GetAllWidgetsOfClass "/Game/Blueprints/Widgets/WBP_DevMenu.WBP_DevMenu_C" false))
  (Default|RegisterPlayerActors (Utilities|Array|Get(acopy) _foundwidgets))
  (Players|RefreshPlayerCameraRefs)
  (CallFunction|HandleGameSave)
  (Variables|/Script/Engine.PlayerController|SetbShowMouseCursor (Game|GetPlayerController 0) true))

(fn UpdateTimer
  (params (Delta%20Time :type Float%20%28double-precision%29))
  ;[1 1 1] Updates minigame timer internally once per frame, updates UI element once per second
  (Variables|Default|SetMinigameTimer (- (Variables|Default|GetMinigameTimer) Delta%20Time))
  (bind _output_get (Variables|Default|SetMinigameUpdateTimer (+ (Variables|Default|GetMinigameUpdateTimer) Delta%20Time)))
  (if (>= _output_get 1.0)
    (UI|Timer|SetTimerText)
    (Math|Float|DecrementFloat (Variables|Default|GetMinigameUpdateTimer))))

(fn ToggleAllPlayersControl
  (params (PlayerControl :type Boolean))
  (bind _outactors (Actor|GetAllActorsOfClass "/Game/Blueprints/Characters/BP_MinigameCharacter.BP_MinigameCharacter_C"))
  (for _array_element _outactors
    (Variables|/Game/Blueprints/Characters/BP_MinigameCharacter.BP_MinigameCharacter_C|SetControlEnabled _array_element PlayerControl)))

(fn SetTimerOpacity
  (params (NewOpacity :type Float%20%28double-precision%29))
  (Default|SetTimerOpacity (Variables|Default|GetTimer) NewOpacity))

(fn SetCountdownOpacity
  (params (NewOpacity :type Float%20%28double-precision%29))
  (Default|SetCountdownOpacity (Variables|Default|GetCountdown) NewOpacity))

(fn TickCountdownStep
  (bind _countdown (Variables|Default|GetCountdown))
  (switch int (Variables|Default|GetCountdownStep)
    (:0
      (Default|SetCountdownText _countdown "2"))
    (:1
      (Default|SetCountdownText _countdown "1"))
    (:2
      (Default|SetCountdownText _countdown "0")))
  (Math|Integer|IncrementInt (Variables|Default|GetCountdownStep)))

(fn SetTimerText
  (bind _timer (Variables|Default|GetTimer))
  (Utilities|IsValid _timer
    (:Is%20Valid
      (Default|SetTimerText _timer (Utilities|Text|ToText(Integer) (Math|Float|Floor (Variables|Default|GetMinigameTimer)))))
    (:Is%20Not%20Valid
      (Development|PrintString "Should have reference to timer but we don't"))))

(fn SetCountdownText
  (params (NewText :type String))
  (Default|SetCountdownText (Variables|Default|GetCountdown) (Utilities|Text|ToText(String) NewText)))

(fn HandleGameSave
  (bind _returnvalue (SaveGame|LoadGamefromSlot "GameSettings"))
  (Utilities|IsValid _returnvalue
    (:Is%20Valid
      (Utilities|Casting|CastToBP_GameSave _returnvalue)
      (Default|LoadSavedParameters (Variables|Default|GetDevMenuRef)))
    (:Is%20Not%20Valid
      (bind _returnvalue_2 (SaveGame|CreateSaveGameObject "/Game/Blueprints/Utilities/BP_GameSave.BP_GameSave_C"))
      (SaveGame|SaveGametoSlot _returnvalue_2 "GameSettings")))
  (return))

(fn SetPlayerMaterial
  (params (PlayerMesh :type Skeletal%20Mesh%20Component%20Object%20Reference) (Index :type Integer))
  (switch int Index
    (:0
      (Rendering|Material|SetMaterial PlayerMesh 0 "/Game/Characters/Mannequins/Materials/Instances/Quinn/MI_Player1Mat_01.MI_Player1Mat_01")
      (Rendering|Material|SetMaterial PlayerMesh 1 "/Game/Characters/Mannequins/Materials/Instances/Quinn/MI_Player1Mat_02.MI_Player1Mat_02"))
    (:1
      (Rendering|Material|SetMaterial PlayerMesh 0 "/Game/Characters/Mannequins/Materials/Instances/Quinn/MI_Player2Mat_01.MI_Player2Mat_01")
      (Rendering|Material|SetMaterial PlayerMesh 1 "/Game/Characters/Mannequins/Materials/Instances/Quinn/MI_Player2Mat_02.MI_Player2Mat_02"))
    (:2
      (Rendering|Material|SetMaterial PlayerMesh 0 "/Game/Characters/Mannequins/Materials/Instances/Quinn/MI_Player3Mat_01.MI_Player3Mat_01")
      (Rendering|Material|SetMaterial PlayerMesh 1 "/Game/Characters/Mannequins/Materials/Instances/Quinn/MI_Player3Mat_02.MI_Player3Mat_02"))
    (:3
      (Rendering|Material|SetMaterial PlayerMesh 0 "/Game/Characters/Mannequins/Materials/Instances/Quinn/MI_Player4Mat_01.MI_Player4Mat_01")
      (Rendering|Material|SetMaterial PlayerMesh 1 "/Game/Characters/Mannequins/Materials/Instances/Quinn/MI_Player4Mat_02.MI_Player4Mat_02"))))

(fn ResetGame
  (bind _asbp_game_instance (Utilities|Casting|CastToBP_GameInstance (Game|GetGameInstance)))
  (bind _output_get (LocalVariables|SetGameInstanceRef _asbp_game_instance))
  (Variables|/Game/Blueprints/Utilities/BP_GameInstance.BP_GameInstance_C|SetCurrRound _output_get 0)
  (for _index (range 0 3)
    (Utilities|Array|SetArrayElem (Variables|/Game/Blueprints/Utilities/BP_GameInstance.BP_GameInstance_C|GetPlayerScores (LocalVariables|GetGameInstanceRef)) _index 0)
    (Utilities|Array|SetArrayElem (Variables|/Game/Blueprints/Utilities/BP_GameInstance.BP_GameInstance_C|GetPrevMinigameRanks (LocalVariables|GetGameInstanceRef)) _index 0)))

(fn SetPlayersVisibilities
  (params (Visible :type Boolean))
  (for _array_element (Variables|Default|GetPlayers)
    (Default|TogglePlayerVisibility _array_element Visible)))

(fn CreateCountdownWidget
  (bind _returnvalue (UserInterface|CreateWidget "/Game/Blueprints/Widgets/WBP_Countdown.WBP_Countdown_C"))
  (bind _output_get (Variables|Default|SetCountdown _returnvalue))
  (UserInterface|Viewport|AddtoViewport _output_get 0))

(fn CreateTimerWidget
  (bind _returnvalue (UserInterface|CreateWidget "/Game/Blueprints/Widgets/WBP_Timer.WBP_Timer_C"))
  (bind _output_get (Variables|Default|SetTimer _returnvalue))
  (UserInterface|Viewport|AddtoViewport _output_get 0))

(fn CreateFadeWidget
  (bind _returnvalue (UserInterface|CreateWidget "/Game/Blueprints/Widgets/WBP_Fade.WBP_Fade_C"))
  (bind _output_get (Variables|Default|SetFade _returnvalue))
  (UserInterface|Viewport|AddtoViewport _output_get 0))

(fn SetFadeOpacity
  (params (Opacity :type Float%20%28double-precision%29))
  (Default|SetFadeOpacity (Variables|Default|GetFade) Opacity))

(fn RefreshPlayerCameraRefs
  (for _array_element (Variables|Default|GetPlayers)
    (Default|RefreshCameraRef _array_element)))

(fn ChangeGameState
  (params (New%20State :type EN_GameState%20Enum :default "NewEnumerator0"))
  (bind _asbp_game_instance (Utilities|Casting|CastToBP_GameInstance (Game|GetGameInstance)))
  (Variables|/Game/Blueprints/Utilities/BP_GameInstance.BP_GameInstance_C|SetCurrGameState _asbp_game_instance New%20State))