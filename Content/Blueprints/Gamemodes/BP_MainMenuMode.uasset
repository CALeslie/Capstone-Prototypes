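; Main menu game mode that shows the menu widget and mouse cursor, sets an initial game state and creates local players in a loop.
; On the first load recorded in the game instance, timelines play two splash screens before fading in the menu; later visits skip straight to the fade.
; A load-hub event fades to black through the widget, then opens the hub level.
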(event Custom|LoadHub_
  (bind _blackfade (Timeline|FadeOutMenu_ PlayFromStart)
    (:Update
      (Default|SetBlackFadeOpacity (Variables|Default|GetUIRef) _blackfade))
    (:Finished
      (Game|OpenLevel(byObjectReference) "/Game/Environments/Levels/HubLevel.HubLevel"))))

(event EventBeginPlay
  (|CallParentFunction)
  (Variables|/Script/Engine.PlayerController|SetbShowMouseCursor (Game|GetPlayerController 0) true)
  (bind _asbp_game_instance (Utilities|Casting|CastToBP_GameInstance (Game|GetGameInstance)))
  (Variables|Default|SetGameInstance_0 _asbp_game_instance)
  (bind _returnvalue (UserInterface|CreateWidget "/Game/Blueprints/Widgets/WBP_MainMenu.WBP_MainMenu_C"))
  (bind _output_get (Variables|Default|SetUIRef _returnvalue))
  (UserInterface|Viewport|AddtoViewport _output_get 0)
  (CallFunction|ChangeGameState "NewEnumerator0")
  (for _index (range 0 3)
    (Class|GameplayStatics|CreatePlayer -1))
  (if (Variables|/Game/Blueprints/Utilities/BP_GameInstance.BP_GameInstance_C|GetFirstLoad (Variables|Default|GetGameInstance_0))
    (bind (_direction _splash1opacity _splash2opacity) (Timeline|ShowSplashScreens_ Play)
      (:Update
        (Default|SetSplashOpacity (Variables|Default|GetUIRef) 0 _splash1opacity)
        (Default|SetSplashOpacity (Variables|Default|GetUIRef) 1 _splash2opacity))
      (:Finished
        (Variables|/Game/Blueprints/Utilities/BP_GameInstance.BP_GameInstance_C|SetFirstLoad (Variables|Default|GetGameInstance_0) false)
        (bind _blackfade (Timeline|FadeInMenu_ PlayFromStart)
          (:Update
            (Default|SetBlackFadeOpacity (Variables|Default|GetUIRef) _blackfade)
            (bind _result (Math|Float|NegateFloat _blackfade)
              (:%20%20
                (Default|SetMainMenuOpacity (Variables|Default|GetUIRef) (+ _result 1.0))))))))
    (else
      (Timeline|FadeInMenu_ PlayFromStart))))

(fn ConstructionScript
  (|CallParentFunction))