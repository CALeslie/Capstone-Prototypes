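; BP_PostGameMode is the post-game mode that announces the winner, the player with the lowest score, then returns to the main menu.
; On BeginPlay it creates fade and countdown widgets and finds the winner from BP_GameInstance's PlayerScores.
; The countdown widget shows the winner text, with timelines driving text and fade opacity.
; After a pause and fade-out, it resets the game and opens the main menu level.
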(event EventBeginPlay
  (|CallParentFunction)
  (CallFunction|CreateFadeWidget)
  (CallFunction|CreateCountdownWidget)
  (bind (_playernum _score) (CallFunction|GetWinningPlayer))
  (CallFunction|SetCountdownText (Utilities|String|Append "P" (Utilities|String|ToString(Integer) _playernum) " is the winner, lowest score of " (Utilities|String|ToString(Integer) _score) " points!"))
  (bind _opacity (Timeline|FadeInWinText_ PlayFromStart)
    (:Update
      (CallFunction|SetCountdownOpacity _opacity)
      (bind _result (Math|Float|NegateFloat _opacity)
        (:%20%20
          (CallFunction|SetFadeOpacity (+ _result 1.0)))))
    (:Finished
      (Utilities|FlowControl|Delay 5.0)
      (bind _opacity_2 (Timeline|FadeOutPostGame_ PlayFromStart)
        (:Update
          (CallFunction|SetFadeOpacity _opacity_2))
        (:Finished
          (CallFunction|SetCountdownOpacity 0.0)
          (CallFunction|ResetGame)
          (Game|OpenLevel(byObjectReference) "/Game/Environments/Levels/MainMenuLevel.MainMenuLevel"))))))

(fn ConstructionScript
  (|CallParentFunction))

(fn GetWinningPlayer
  (bind _asbp_game_instance (Utilities|Casting|CastToBP_GameInstance (Game|GetGameInstance)))
  (for (_array_element _array_index) (Variables|/Game/Blueprints/Utilities/BP_GameInstance.BP_GameInstance_C|GetPlayerScores _asbp_game_instance)
    (if (< _array_element (LocalVariables|GetLowestScore))
      (LocalVariables|SetLowestScore _array_element)
      (LocalVariables|SetLowestScoreIndex _array_index)))
  (return (+ (LocalVariables|GetLowestScoreIndex) 1) (LocalVariables|GetLowestScore)))