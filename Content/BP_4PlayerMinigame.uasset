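; Game mode for a local four-player minigame that spawns and possesses a BP_MinigameCharacter for each player.
; One second after BeginPlay, SpawnPlayers shuffles the PlayerStarts, creates a local player per start, and destroys each start used.
; It then restarts player 0 as cleanup for the default controller and has WBP_MovementControls register the player actors.
; PostLogin destroys any controller that logs in.
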(event EventBeginPlay
  (Variables|/Script/Engine.PlayerController|SetbShowMouseCursor (Game|GetPlayerController 0) true)
  (Utilities|FlowControl|Delay 1.0)
  (CallFunction|SpawnPlayers))

(event EventTick
  (params (DeltaSeconds :type Float%20%28single-precision%29)))

(event EventHandleStartingNewPlayer
  (params (NewPlayer :type Player%20Controller%20Object%20Reference)))

(event EventPostLogin
  (params (NewPlayer :type Player%20Controller%20Object%20Reference))
  (Actor|DestroyActor NewPlayer))

(fn ConstructionScript)

(fn SpawnPlayers
  ;[1 1 1] Gathers all player spawns in a randomized array and iterates over them (randomizes spawn locations, allows for more than 4 spawns)
  (bind _outactors (Actor|GetAllActorsOfClass "/Script/Engine.PlayerStart"))
  (bind _output_get (LocalVariables|SetPlayerStarts _outactors))
  (Utilities|Array|Shuffle _output_get)
  (for (_array_element _array_index) _output_get
    ;[1 1 1] Creates player controller, if valid spawns character pawn at player start entity and then possesses pawn with that controller
    (bind _returnvalue (Class|GameplayStatics|CreatePlayer _array_index))
    (if (Utilities|IsValid _returnvalue)
      (bind _returnvalue_2 (Game|SpawnActorfromClass "/Game/Minigame/Blueprints/BP_MinigameCharacter.BP_MinigameCharacter_C" (Transformation|GetActorTransform _array_element) "AlwaysSpawn" "MultiplyWithRoot" 0 0))
      (Pawn|Possess _returnvalue _returnvalue_2)
      (Actor|DestroyActor _array_element) ; Destroys player starts after using to ensure multiple players aren't spawned on same ones
    ))
  ;[1 1 1] Required to clean up default spawned controller
  (Variables|Default|SetDefaultPawnClass "/Game/Minigame/Blueprints/BP_MinigameCharacter.BP_MinigameCharacter_C")
  (Class|GameModeBase|RestartPlayer (Game|GetPlayerController 0))
  (bind _foundwidgets (Widget|GetAllWidgetsOfClass "/Game/Minigame/Blueprints/WBP_MovementControls.WBP_MovementControls_C" true))
  (Default|RegisterPlayerActors (Utilities|Array|Get(acopy) _foundwidgets)))