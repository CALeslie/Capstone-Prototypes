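; Bed actor for the HS minigame that plays an opening animation on its Bed component.
; The PlayOpenAnim event restarts the OpenAnimation timeline, which drives the bed's relative roll and Z position on each update.
; It has no other active logic, as BeginPlay, overlap and Tick are disabled stubs.
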(event EventBeginPlay
  (|CallParentFunction) ; This node is disabled and will not be called.\nDrag off pins to build functionality.
)

(event Collision|EventActorBeginOverlap
  (params (OtherActor :type Actor%20Object%20Reference))
  (|CallParentFunction OtherActor) ; This node is disabled and will not be called.\nDrag off pins to build functionality.
)

(event EventTick
  (params (DeltaSeconds :type Float%20%28single-precision%29))
  (|CallParentFunction DeltaSeconds) ; This node is disabled and will not be called.\nDrag off pins to build functionality.
)

(event EventPlayOpenAnim
  (bind _bed (Variables|Default|GetBed))
  (bind (_direction _bedrotationx _bedpositionz) (Timeline|OpenAnimation PlayFromStart)
    (:Update
      (Transformation|SetRelativeRotation _bed (Math|Rotator|MakeRotator _bedrotationx 0.0 0.0) false false)
      (Transformation|SetRelativeLocation _bed (Math|Vector|MakeVector 0.0 0.0 _bedpositionz) false false))))

(fn ConstructionScript
  (|CallParentFunction))