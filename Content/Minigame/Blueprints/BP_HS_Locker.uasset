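; BP_HS_Locker is a minigame locker actor with a door that animates open.
; PlayOpenAnim runs a timeline that drives the Door component's yaw.
; PlayPermOpenAnim sets the PermOpen flag and runs a second timeline that rotates the door on all three axes.
; Both events restart their timeline from the start; nothing in this graph calls them or reads the flag.
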(event EventBeginPlay
  (|CallParentFunction) ; This node is disabled and will not be called.\nDrag off pins to build functionality.
)

(event Collision|EventActorBeginOverlap
  (params (OtherActor :type Actor%20Object%20Reference))
  (|CallParentFunction OtherActor) ; This node is disabled and will not be called.\nDrag off pins to build functionality.
)

(event EventTick
  (params (DeltaSeconds :type Float%20%28single-precision%29))
  (|CallParentFunction DeltaSeconds) ; This node is disabled and will not be called.\nDrag off pins to build functionality.
)

(event EventPlayOpenAnim
  (bind _doorrotationz (Timeline|OpenAnimation PlayFromStart)
    (:Update
      (Transformation|SetRelativeRotation (Variables|Default|GetDoor) (Math|Rotator|MakeRotator 0.0 0.0 _doorrotationz) false false))))

(event EventPlayPermOpenAnim
  (Variables|Default|SetPermOpen true)
  (bind (_direction _doorrotationz _doorrotationy _doorrotationx) (Timeline|PermOpenAnimatino PlayFromStart)
    (:Update
      (Transformation|SetRelativeRotation (Variables|Default|GetDoor) (Math|Rotator|MakeRotator _doorrotationx _doorrotationy _doorrotationz) false false))))

(fn ConstructionScript
  (|CallParentFunction))