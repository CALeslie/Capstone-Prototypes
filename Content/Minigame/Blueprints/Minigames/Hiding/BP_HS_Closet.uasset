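; BP_HS_Closet is a two-door closet for the hiding minigame, with animated opening doors.
; Two externally called events each play a timeline from the start, driving the relative yaw of the left and right doors.
; PlayOpenAnim runs the regular open animation, while PlayPermOpenAnim also sets the PermOpen flag and plays a separate permanent-open timeline.
; The closet only exposes this state and animation, with no hiding or trigger logic of its own.
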(event EventBeginPlay
  (|CallParentFunction) ; This node is disabled and will not be called.\nDrag off pins to build functionality.
)

(event Collision|EventActorBeginOverlap
  (params (OtherActor :type Actor%20Object%20Reference))
  (|CallParentFunction OtherActor) ; This node is disabled and will not be called.\nDrag off pins to build functionality.
)

(event EventTick
  (params (DeltaSeconds :type Float%20%28single-precision%29))
  (|CallParentFunction DeltaSeconds) ; This node is disabled and will not be called.\nDrag off pins to build functionality.
)

(event EventPlayOpenAnim
  (bind (_direction _ldoorrotation _rdoorrotation) (Timeline|OpenAnim PlayFromStart)
    (:Update
      (Transformation|SetRelativeRotation (Variables|Default|GetDoorLeft) (Math|Rotator|MakeRotator 0.0 0.0 _ldoorrotation) false false)
      (Transformation|SetRelativeRotation (Variables|Default|GetDoorRight) (Math|Rotator|MakeRotator 0.0 0.0 _rdoorrotation) false false))))

(event EventPlayPermOpenAnim
  (Variables|Default|SetPermOpen true)
  (bind (_direction _ldoorrotation _rdoorrotation) (Timeline|PermOpenAnim PlayFromStart)
    (:Update
      (Transformation|SetRelativeRotation (Variables|Default|GetDoorLeft) (Math|Rotator|MakeRotator 0.0 0.0 _ldoorrotation) false false)
      (Transformation|SetRelativeRotation (Variables|Default|GetDoorRight) (Math|Rotator|MakeRotator 0.0 0.0 _rdoorrotation) false false))))

(fn ConstructionScript
  (|CallParentFunction))