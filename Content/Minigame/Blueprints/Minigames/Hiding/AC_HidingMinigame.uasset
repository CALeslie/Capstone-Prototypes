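; Actor component that runs the rules of the Hiding minigame, where players hide from an enemy over repeated rounds.
; Setup finds the door, hiding spots and enemy controller, primes the hide timer and resets players, who later teleport to shuffled starts.
; Status changes toggle player control, and elimination delegates to the enemy based on whether anyone is unhidden.
; Between rounds it reveals survivors and frees spots, while catches adjust ranks by round count.
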(event EventBeginPlay)

(event EventTick
  (params (DeltaSeconds :type Float%20%28single-precision%29)))

(fn MinigameSetup
  (params (GameModeRef :type BP%20Minigame%20Mode%20Object%20Reference))
  (bind _timetohide (Variables|Default|GetTimeToHide))
  (bind _playerranks (Variables|Default|GetPlayerRanks))
  (Utilities|IsValid (Variables|Default|GetGameModeRef)
    (:Is%20Valid
      _)
    (:Is%20Not%20Valid
      (Variables|Default|SetGameModeRef GameModeRef)))
  (Variables|Default|SetMinigameStatus "NewEnumerator0")
  (bind _returnvalue (Actor|GetActorOfClass "/Game/Minigame/Blueprints/Minigames/Hiding/BP_Hide_Door.BP_Hide_Door_C"))
  (Variables|Default|SetEnemyDoor _returnvalue)
  (bind _outactors (Actor|GetAllActorsOfClass "/Game/Minigame/Blueprints/Minigames/Hiding/BP_HidingSpot.BP_HidingSpot_C"))
  (Variables|Default|SetHidingSpots _outactors)
  (Variables|Default|SetCaughtPlayers (Utilities|Array|MakeArray 0))
  (bind _outactors_2 (Actor|GetAllActorsOfClass "/Game/Minigame/Blueprints/Minigames/Hiding/BP_EnemyController.BP_EnemyController_C"))
  (bind _output_get (Variables|Default|SetEnemy (Utilities|Array|Get(acopy) _outactors_2)))
  (bind _output_get_2 (Variables|/Game/Minigame/Blueprints/Minigames/Hiding/BP_EnemyController.BP_EnemyController_C|SetMinigameModeRef _output_get (Variables|Default|GetGameModeRef)))
  (Variables|/Game/Minigame/Blueprints/BP_MinigameMode.BP_MinigameMode_C|SetMinigameTimer _output_get_2 _timetohide)
  (Default|SetTimerText _output_get_2)
  (Variables|/Game/Minigame/Blueprints/BP_MinigameMode.BP_MinigameMode_C|SetMinigameTimer _output_get_2 (+ _timetohide 1.0))
  (Default|SetTimerOpacity (Variables|/Game/Minigame/Blueprints/BP_MinigameMode.BP_MinigameMode_C|GetMinigameUIRef (Variables|Default|GetGameModeRef)) 1.0)
  (Default|SetCountdownOpacity (Variables|/Game/Minigame/Blueprints/BP_MinigameMode.BP_MinigameMode_C|GetMinigameUIRef (Variables|Default|GetGameModeRef)) 0.0)
  (Variables|/Game/Minigame/Blueprints/BP_MinigameMode.BP_MinigameMode_C|SetCountdownStep (Variables|Default|GetGameModeRef) 0)
  (for _array_element (Variables|/Game/Minigame/Blueprints/BP_MinigameMode.BP_MinigameMode_C|GetPlayers (Variables|Default|GetGameModeRef))
    (Default|RefreshCameraRef _array_element)
    (Variables|/Game/Minigame/Blueprints/BP_MinigameCharacter.BP_MinigameCharacter_C|SetCaught _array_element false)
    (Variables|/Game/Minigame/Blueprints/BP_MinigameCharacter.BP_MinigameCharacter_C|SetHidden _array_element false)
    (for (_ _array_index) _playerranks
      (Utilities|Array|SetArrayElem _playerranks _array_index 4))))

(fn UpdateMinigameStatus
  (params (New%20Status :type EN_HidingMinigameStatus%20Enum :default "NewEnumerator0"))
  (bind _gamemoderef (Variables|Default|GetGameModeRef))
  (bind _output_get (Variables|Default|SetMinigameStatus New%20Status))
  (switch Utilities|FlowControl|Switch|SwitchonEN_HidingMinigameStatus _output_get
    (:NewEnumerator0
      (Default|ToggleAllPlayersControl _gamemoderef false :!label _label))
    (:NewEnumerator1
      (Default|ToggleAllPlayersControl _gamemoderef true))
    (:NewEnumerator3
      (goto _label))
    (:NewEnumerator2
      (goto _label))))

(fn EliminatePlayers
  (bind _enemy (Variables|Default|GetEnemy))
  (for _array_element (Variables|/Game/Minigame/Blueprints/BP_MinigameMode.BP_MinigameMode_C|GetPlayers (Variables|Default|GetGameModeRef))
    (if (not (Variables|/Game/Minigame/Blueprints/BP_MinigameCharacter.BP_MinigameCharacter_C|GetCaught _array_element))
      (if (not (Variables|/Game/Minigame/Blueprints/BP_MinigameCharacter.BP_MinigameCharacter_C|GetHidden _array_element))
        (LocalVariables|SetPlayersNotHidden true))))
  (if (LocalVariables|GetPlayersNotHidden)
    (Default|EliminatePlayers _enemy)
    (else
      (Default|EliminatePlayer _enemy))))

(fn OpenDoor
  (Default|EventOpenDoor (Variables|Default|GetEnemyDoor)))

(fn SetupEnemyandPlayers
  (Default|SetupEnemy (Variables|Default|GetEnemy) (Variables|/Game/Minigame/Blueprints/BP_MinigameMode.BP_MinigameMode_C|GetPlayers (Variables|Default|GetGameModeRef)))
  (bind _outactors (Actor|GetAllActorsOfClass "/Game/Minigame/Blueprints/BP_PlayerStart.BP_PlayerStart_C"))
  (bind _output_get (LocalVariables|SetPlayerStarts _outactors))
  (Utilities|Array|Shuffle _output_get)
  (for (_array_element _array_index) (LocalVariables|GetPlayerStarts)
    (Transformation|SetActorLocationAndRotation (Utilities|Array|Get(acopy) (Variables|/Game/Minigame/Blueprints/BP_MinigameMode.BP_MinigameMode_C|GetPlayers (Variables|Default|GetGameModeRef)) _array_index) (Math|Vector|MakeVector (.x (Transformation|GetActorLocation _array_element)) (.y (Transformation|GetActorLocation _array_element)) (+ (.z (Transformation|GetActorLocation _array_element)) 30.62)) (Transformation|GetActorRotation _array_element) false true)
    (Default|TogglePlayerVisibility (Utilities|Array|Get(acopy) (Variables|/Game/Minigame/Blueprints/BP_MinigameMode.BP_MinigameMode_C|GetPlayers (Variables|Default|GetGameModeRef)) _array_index) true)))

(fn ReshowPlayer
  (params (PlayerRef :type BP%20Minigame%20Character%20Object%20Reference))
  (bind _output_get (LocalVariables|SetPlayer PlayerRef))
  (Transformation|SetActorRotation _output_get (Math|Rotator|MakeRotator 0.0 0.0 (+ (.yaw (Transformation|GetActorRotation (LocalVariables|GetPlayer))) 1.8e+02)))
  (Default|TogglePlayerVisibility (LocalVariables|GetPlayer) true)
  (if (Variables|/Game/Minigame/Blueprints/BP_MinigameCharacter.BP_MinigameCharacter_C|GetCaught (LocalVariables|GetPlayer))
    _
    (else
      (Variables|/Game/Minigame/Blueprints/BP_MinigameCharacter.BP_MinigameCharacter_C|SetHidden (LocalVariables|GetPlayer) false)
      (Variables|/Game/Minigame/Blueprints/BP_MinigameCharacter.BP_MinigameCharacter_C|SetControlEnabled (LocalVariables|GetPlayer) true)))
  (Default|PlayOpenAnim (Variables|/Game/Minigame/Blueprints/BP_MinigameCharacter.BP_MinigameCharacter_C|GetHidingSpotRef (LocalVariables|GetPlayer))))

(fn ReshowPlayers
  (for _array_element (Variables|/Game/Minigame/Blueprints/BP_MinigameMode.BP_MinigameMode_C|GetPlayers (Variables|Default|GetGameModeRef))
    (if (not (Variables|/Game/Minigame/Blueprints/BP_MinigameCharacter.BP_MinigameCharacter_C|GetCaught _array_element))
      (CallFunction|ReshowPlayer _array_element)))
  (Math|Integer|IncrementInt (Variables|Default|GetMinigameRounds)))

(fn CheckPlayersLeft
  (for _array_element (Variables|/Game/Minigame/Blueprints/BP_MinigameMode.BP_MinigameMode_C|GetPlayers (Variables|Default|GetGameModeRef))
    (if (not (Variables|/Game/Minigame/Blueprints/BP_MinigameCharacter.BP_MinigameCharacter_C|GetCaught _array_element))
      (Math|Integer|IncrementInt (LocalVariables|GetNumPlayersLeft))))
  (return (> (LocalVariables|GetNumPlayersLeft) 1)))

(fn UpdateHidingSpots
  (for _array_element (Variables|Default|GetHidingSpots)
    (Variables|/Game/Minigame/Blueprints/Minigames/Hiding/BP_HidingSpot.BP_HidingSpot_C|SetUsed _array_element false)))

(fn CatchPlayer
  (params (Player :type BP%20Minigame%20Character%20Object%20Reference))
  (bind _playerid (Variables|/Game/Minigame/Blueprints/BP_MinigameCharacter.BP_MinigameCharacter_C|GetPlayerID Player))
  (bind _playerranks (Variables|Default|GetPlayerRanks))
  (Default|PlayerCaught Player)
  (Utilities|Array|AppendArray (Variables|Default|GetCaughtPlayers) (Utilities|Array|MakeArray Player))
  (Utilities|Array|SetArrayElem _playerranks _playerid (+ (Utilities|Array|Get(acopy) _playerranks _playerid) (Variables|Default|GetMinigameRounds))))