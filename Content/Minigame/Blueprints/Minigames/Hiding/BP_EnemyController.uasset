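; Enemy controller for the hiding minigame that walks the enemy in to catch players.
; EliminatePlayers chases every uncaught, unhidden player in shuffled order, while EliminatePlayer opens one random uncaught player's hiding spot and removes them.
; Both chain AIMoveTo calls, counting failed moves as arrivals, then share a TurnAround timeline exit that eases walk speed and notifies the minigame mode.
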(event Custom|EliminatePlayers
  (bind _enemymovement (Variables|Default|GetEnemyMovement))
  (bind _enemymovement_2 (Variables|Default|GetEnemyMovement))
  (Variables|Default|SetPlayersToEliminate (Utilities|Array|MakeArray))
  (Variables|/Script/Engine.CharacterMovementComponent|SetMaxWalkSpeed (Variables|Default|GetEnemyMovement) 1.5e+02)
  (AI|AIMoveTo 0 "850.000000,0.000000,117.500000" 0 -1.0 "Default" "Default" true true
    (:OnMoveFinished
      (Variables|/Script/Engine.CharacterMovementComponent|SetMaxWalkSpeed _enemymovement 6e+02)
      (Variables|/Script/Engine.CharacterMovementComponent|SetRotationRate _enemymovement "0.000000,240.000000,0.000000")
      (Utilities|FlowControl|Delay 1.0)
      (for _array_element (Variables|Default|GetPlayers)
        (bind _result (CallFunction|IsPlayerValidTarget _array_element))
        (if _result
          (Utilities|Array|AppendArray (Variables|Default|GetPlayersToEliminate) (Utilities|Array|MakeArray _array_element))))
      (Utilities|Array|Shuffle (Variables|Default|GetPlayersToEliminate))
      (Variables|Default|SetCurrentPlayerIndex 0)
      (AI|AIMoveTo 0 "0, 0, 0" (Utilities|Array|Get(acopy) (Variables|Default|GetPlayersToEliminate) (Variables|Default|GetCurrentPlayerIndex)) -1.0 "Default" "Enable" true true false "Default" "Disable"
        (:OnRequestFailed
          _)
        (:OnMoveFinished
          _))
      (Utilities|FlowControl|Delay 0.5)
      (Default|PlayerCaught (Utilities|Array|Get(acopy) (Variables|Default|GetPlayersToEliminate) (Variables|Default|GetCurrentPlayerIndex)))
      (bind _result_2 (Math|Integer|IncrementInt (Variables|Default|GetCurrentPlayerIndex))
        (:%20%20
          (if (>= _result_2 (Utilities|Array|Length (Variables|Default|GetPlayersToEliminate)))
            (Variables|/Script/Engine.CharacterMovementComponent|SetMaxWalkSpeed _enemymovement_2 1e+01)
            (Variables|/Script/Engine.CharacterMovementComponent|SetRotationRate _enemymovement_2 "0.000000,150.000000,0.000000")
            (bind _walkspeed (Timeline|TurnAround PlayFromStart)
              (:Update
                (Variables|/Script/Engine.CharacterMovementComponent|SetMaxWalkSpeed (Variables|Default|GetEnemyMovement) _walkspeed))
              (:StartWalkingEvent
                (AI|AIMoveTo 0 "900.000000,0.000000,117.500000" 0 -1.0 "Default" "Default" true true
                  (:OnMoveFinished
                    (Default|EliminationFinished (Variables|Default|GetMinigameModeRef))
                    (AI|AIMoveTo 0 "1500.000000,0.000000,117.500000" 0 -1.0 "Default" "Default" true true
                      (:OnMoveFinished
                        (Utilities|FlowControl|Delay 4.0)
                        (AI|AIMoveTo 0 "1017.000000,0.000000,117.500000" 0 -1.0 "Default" "Default" true true)))))))
            (else
              (CallFunction|MovetoNextActor))))))))

(event Custom|EliminatePlayer
  (bind _enemymovement (Variables|Default|GetEnemyMovement))
  (bind _enemymovement_2 (Variables|Default|GetEnemyMovement))
  (Variables|Default|SetPlayersToEliminate (Utilities|Array|MakeArray))
  (Variables|/Script/Engine.CharacterMovementComponent|SetMaxWalkSpeed (Variables|Default|GetEnemyMovement) 1.5e+02)
  (AI|AIMoveTo 0 "500.000000,0.000000,117.500000" 0 -1.0 "Default" "Default" true true
    (:OnMoveFinished
      (Variables|/Script/Engine.CharacterMovementComponent|SetMaxWalkSpeed _enemymovement 6e+02)
      (Variables|/Script/Engine.CharacterMovementComponent|SetRotationRate _enemymovement "0.000000,240.000000,0.000000")
      (Utilities|FlowControl|Delay 1.0)
      (for _array_element (Variables|Default|GetPlayers)
        (if (not (Variables|/Game/Minigame/Blueprints/BP_MinigameCharacter.BP_MinigameCharacter_C|GetCaught _array_element))
          (Utilities|Array|AppendArray (Variables|Default|GetPlayersToEliminate) (Utilities|Array|MakeArray _array_element))))
      (Utilities|Array|Shuffle (Variables|Default|GetPlayersToEliminate))
      (AI|AIMoveTo 0 "0, 0, 0" (Utilities|Array|Get(acopy) (Variables|Default|GetPlayersToEliminate)) -1.0 "Default" "Enable" true true false "Default" "Disable"
        (:OnRequestFailed
          _)
        (:OnMoveFinished
          _))
      (Utilities|FlowControl|Delay 0.5)
      (Default|PlayPermOpenAnim (Variables|/Game/Minigame/Blueprints/BP_MinigameCharacter.BP_MinigameCharacter_C|GetHidingSpotRef (Utilities|Array|Get(acopy) (Variables|Default|GetPlayersToEliminate))))
      (Variables|/Game/Minigame/Blueprints/BP_MinigameCharacter.BP_MinigameCharacter_C|SetCaught (Utilities|Array|Get(acopy) (Variables|Default|GetPlayersToEliminate)) true)
      (Default|ReshowHiddenPlayer (Utilities|Array|Get(acopy) (Variables|Default|GetPlayersToEliminate)))
      (Utilities|FlowControl|Delay 1.0)
      (Default|CatchPlayer (Variables|/Game/Minigame/Blueprints/BP_MinigameMode.BP_MinigameMode_C|GetAC_HidingMinigame (Variables|Default|GetMinigameModeRef)) (Utilities|Array|Get(acopy) (Variables|Default|GetPlayersToEliminate)))
      (Variables|/Script/Engine.CharacterMovementComponent|SetMaxWalkSpeed _enemymovement_2 1e+01)
      (Variables|/Script/Engine.CharacterMovementComponent|SetRotationRate _enemymovement_2 "0.000000,150.000000,0.000000")
      (bind _walkspeed (Timeline|TurnAround PlayFromStart)
        (:Update
          (Variables|/Script/Engine.CharacterMovementComponent|SetMaxWalkSpeed (Variables|Default|GetEnemyMovement) _walkspeed))
        (:StartWalkingEvent
          (AI|AIMoveTo 0 "900.000000,0.000000,117.500000" 0 -1.0 "Default" "Default" true true
            (:OnMoveFinished
              (Default|EliminationFinished (Variables|Default|GetMinigameModeRef))
              (AI|AIMoveTo 0 "1500.000000,0.000000,117.500000" 0 -1.0 "Default" "Default" true true
                (:OnMoveFinished
                  (Utilities|FlowControl|Delay 4.0)
                  (AI|AIMoveTo 0 "1017.000000,0.000000,117.500000" 0 -1.0 "Default" "Default" true true))))))))))

(event Custom|SetupEnemy
  (params (Players :type Array%20of%20BP%20Minigame%20Character%20Object%20References))
  (Variables|Default|SetPlayers Players)
  (bind _returnvalue (Actor|GetActorOfClass "/Game/Minigame/Blueprints/Minigames/Hiding/BP_HidingMinigameEnemy.BP_HidingMinigameEnemy_C"))
  (Variables|Default|SetEnemyMovement (Variables|/Script/Engine.Character|GetCharacterMovement _returnvalue)))

(event Custom|MoveToNextActor
  (bind _currentplayerindex (Variables|Default|GetCurrentPlayerIndex))
  (bind _enemymovement (Variables|Default|GetEnemyMovement))
  (bind _playerstoeliminate (Variables|Default|GetPlayersToEliminate))
  (bind _output (Utilities|Array|Get(acopy) _playerstoeliminate _currentplayerindex))
  (AI|AIMoveTo 0 "0, 0, 0" _output -1.0 "Default" "Enable" true true false "Default" "Disable"
    (:OnRequestFailed
      _)
    (:OnMoveFinished
      _))
  (Utilities|FlowControl|Delay 0.5)
  (Default|PlayerCaught _output)
  (bind _result (Math|Integer|IncrementInt (Variables|Default|GetCurrentPlayerIndex))
    (:%20%20
      (if (>= _result (Utilities|Array|Length (Variables|Default|GetPlayersToEliminate)))
        (Variables|/Script/Engine.CharacterMovementComponent|SetMaxWalkSpeed _enemymovement 1e+01)
        (Variables|/Script/Engine.CharacterMovementComponent|SetRotationRate _enemymovement "0.000000,150.000000,0.000000")
        (bind _walkspeed (Timeline|TurnAround PlayFromStart)
          (:Update
            (Variables|/Script/Engine.CharacterMovementComponent|SetMaxWalkSpeed (Variables|Default|GetEnemyMovement) _walkspeed))
          (:StartWalkingEvent
            (AI|AIMoveTo 0 "900.000000,0.000000,117.500000" 0 -1.0 "Default" "Default" true true
              (:OnMoveFinished
                (Default|EliminationFinished (Variables|Default|GetMinigameModeRef))
                (AI|AIMoveTo 0 "1500.000000,0.000000,117.500000" 0 -1.0 "Default" "Default" true true
                  (:OnMoveFinished
                    (Utilities|FlowControl|Delay 4.0)
                    (AI|AIMoveTo 0 "1017.000000,0.000000,117.500000" 0 -1.0 "Default" "Default" true true)))))))
        (else
          (CallFunction|MovetoNextActor))))))

(event EventBeginPlay)

(event EventTick
  (params (DeltaSeconds :type Float%20%28single-precision%29)))

(fn ConstructionScript)

(fn IsPlayerValidTarget
  (params (Player%20Ref :type BP%20Minigame%20Character%20Object%20Reference))
  (if (Variables|/Game/Minigame/Blueprints/BP_MinigameCharacter.BP_MinigameCharacter_C|GetCaught Player%20Ref)
    (LocalVariables|SetValidTarget false :!label _label)
    (elif (Variables|/Game/Minigame/Blueprints/BP_MinigameCharacter.BP_MinigameCharacter_C|GetHidden Player%20Ref)
      (goto _label)
      (else
        (LocalVariables|SetValidTarget true))))
  (return (LocalVariables|GetValidTarget)))