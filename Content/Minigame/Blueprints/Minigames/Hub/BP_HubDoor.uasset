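; BP_HubDoor is a double door in the minigame hub that represents a next minigame type, displayed on its connected text.
; Overlap events track nearby minigame characters found in the hub component's last-place list, which is fetched from BP_MinigameMode and cached.
; The connected light turns on while eligible players are nearby and off when the last leaves.
; A separate OpenDoor event swings both panels using a timeline.
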(event Custom|OpenDoor
  (bind (_direction _leftdoorrotation _rightdoorrotation) (Timeline|OpenDoorAnim PlayFromStart)
    (:Update
      (Transformation|SetRelativeRotation (Variables|Default|GetDoorLeft) (Math|Rotator|MakeRotator 0.0 0.0 _leftdoorrotation) false false)
      (Transformation|SetRelativeRotation (Variables|Default|GetDoorRight) (Math|Rotator|MakeRotator 0.0 0.0 _rightdoorrotation) false false))))

(event EventBeginPlay)

(event Collision|EventActorBeginOverlap
  (params (OtherActor :type Actor%20Object%20Reference))
  (bind _asbp_minigame_character (Utilities|Casting|CastToBP_MinigameCharacter OtherActor))
  (bind (_result _player) (CallFunction|LastPlaceCheck _asbp_minigame_character))
  (if _result
    (CallFunction|AddEligiblePlayer _player)))

(event EventTick
  (params (DeltaSeconds :type Float%20%28single-precision%29)))

(event Collision|EventActorEndOverlap
  (params (OtherActor :type Actor%20Object%20Reference))
  (bind _asbp_minigame_character (Utilities|Casting|CastToBP_MinigameCharacter OtherActor))
  (bind (_result _player) (CallFunction|LastPlaceCheck _asbp_minigame_character))
  (if _result
    (CallFunction|RemoveEligiblePlayer _player)))

(fn ConstructionScript)

(fn LastPlaceCheck
  (params (Player%20Ref :type BP%20Minigame%20Character%20Object%20Reference))
  (LocalVariables|SetPlayerLocalRef Player%20Ref)
  (Utilities|IsValid (Variables|Default|GetHubACRef)
    (:Is%20Valid
      _)
    (:Is%20Not%20Valid
      (bind _returnvalue (Actor|GetActorOfClass "/Game/Minigame/Blueprints/BP_MinigameMode.BP_MinigameMode_C"))
      (Variables|Default|SetHubACRef (Variables|/Game/Minigame/Blueprints/BP_MinigameMode.BP_MinigameMode_C|GetAC_Hub _returnvalue))))
  (if (> (Utilities|Array|FindItem (Variables|/Game/AC_HubMode.AC_HubMode_C|GetLastPlacePlayers (Variables|Default|GetHubACRef)) (LocalVariables|GetPlayerLocalRef)) -1)
    (return true (LocalVariables|GetPlayerLocalRef))
    (else
      (return false (LocalVariables|GetPlayerLocalRef)))))

(fn AddEligiblePlayer
  (params (Player :type BP%20Minigame%20Character%20Object%20Reference))
  (Default|Turnon (Variables|Default|GetConnectedLight))
  (Utilities|Array|AppendArray (Variables|Default|GetEligiblePlayersNearby) (Utilities|Array|MakeArray Player)))

(fn RemoveEligiblePlayer
  (params (PlayerRef :type BP%20Minigame%20Character%20Object%20Reference))
  (bind _eligibleplayersnearby (Variables|Default|GetEligiblePlayersNearby))
  (Utilities|Array|RemoveItem _eligibleplayersnearby PlayerRef)
  (if (< (Utilities|Array|Length _eligibleplayersnearby) 1)
    (Default|TurnOff (Variables|Default|GetConnectedLight))))

(fn TurnOffLight
  (Default|TurnOff (Variables|Default|GetConnectedLight)))

(fn TurnonLight
  (Default|Turnon (Variables|Default|GetConnectedLight)))

(fn SetMinigameType
  (params (MinigameType :type EN_HubDoorType%20Enum :default "NewEnumerator0"))
  (Variables|Default|SetNextMinigameType MinigameType)
  (Rendering|Components|TextRender|SetText (Variables|/Script/Engine.TextRenderActor|GetTextRender (Variables|Default|GetConnectedText)) (Utilities|Text|ToText(String) (Utilities|String|EnumtoString MinigameType))))