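; Hub mode component for the minigame hub, which places players at shuffled starts and picks the next minigame.
; Setup fills the scoreboards, randomly assigns minigame types to doors and finds last-place players, taken as those with the highest score.
; Next-game selection randomly picks among doors with eligible players nearby, or any door if none.
; The chosen door opens and its minigame loads through the game mode.
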(event EventBeginPlay)

(event EventTick
  (params (DeltaSeconds :type Float%20%28single-precision%29)))

(fn SetUpPlayers
  (bind _outactors (Actor|GetAllActorsOfClass "/Game/Minigame/Blueprints/BP_PlayerStart.BP_PlayerStart_C"))
  (bind _output_get (LocalVariables|SetPlayerStarts _outactors))
  (Utilities|Array|Shuffle _output_get)
  (for (_array_element _array_index) (LocalVariables|GetPlayerStarts)
    (Transformation|SetActorLocationAndRotation (Utilities|Array|Get(acopy) (Variables|/Game/Minigame/Blueprints/BP_MinigameMode.BP_MinigameMode_C|GetPlayers (Variables|Default|GetGameModeRef)) _array_index) (Math|Vector|MakeVector (.x (Transformation|GetActorLocation _array_element)) (.y (Transformation|GetActorLocation _array_element)) (+ (.z (Transformation|GetActorLocation _array_element)) 30.62)) (Transformation|GetActorRotation _array_element) false true)
    (Default|TogglePlayerVisibility (Utilities|Array|Get(acopy) (Variables|/Game/Minigame/Blueprints/BP_MinigameMode.BP_MinigameMode_C|GetPlayers (Variables|Default|GetGameModeRef)) _array_index) true)
    (Default|RefreshCameraRef (Utilities|Array|Get(acopy) (Variables|/Game/Minigame/Blueprints/BP_MinigameMode.BP_MinigameMode_C|GetPlayers (Variables|Default|GetGameModeRef)) _array_index))))

(fn HubSetup
  (params (GameModeRef :type BP%20Minigame%20Mode%20Object%20Reference))
  (Utilities|IsValid (Variables|Default|GetGameModeRef)
    (:Is%20Valid
      _)
    (:Is%20Not%20Valid
      (Variables|Default|SetGameModeRef GameModeRef)))
  (CallFunction|SetLastPlacePlayers)
  (bind _outactors (Actor|GetAllActorsOfClass "/Game/Minigame/Blueprints/Minigames/Hub/BP_HubDoor.BP_HubDoor_C"))
  (Variables|Default|SetHubDoors _outactors)
  (bind _outactors_2 (Actor|GetAllActorsOfClass "/Game/Minigame/Blueprints/BP_SpotLightControl.BP_SpotLightControl_C"))
  (Variables|Default|SetHubDoorLights _outactors_2)
  (CallFunction|AssignMinigamestoDoors)
  (Variables|Default|SetHubStatus "NewEnumerator0")
  (bind _outactors_3 (Actor|GetAllActorsOfClass "/Game/Minigame/Blueprints/Minigames/Hub/BP_ScoreBoard.BP_ScoreBoard_C"))
  (bind _output_get (Variables|Default|SetScoreboards _outactors_3))
  (for (_array_element _array_index) (Variables|/Game/Minigame/Blueprints/BP_MinigameMode.BP_MinigameMode_C|GetPlayerScores (Variables|Default|GetGameModeRef))
    (Default|SetPlayerScore (Utilities|Array|Get(acopy) _output_get) _array_index _array_element)
    (Default|SetPlayerScore (Utilities|Array|Get(acopy) _output_get 1) _array_index _array_element)))

(fn SetLastPlacePlayers
  (bind _lastplaceplayers (Variables|Default|GetLastPlacePlayers))
  (for (_array_element _array_index) (Variables|/Game/Minigame/Blueprints/BP_MinigameMode.BP_MinigameMode_C|GetPlayerScores (Variables|Default|GetGameModeRef))
    (if (> _array_element (LocalVariables|GetLastPlaceScore))
      (LocalVariables|SetLastPlaceScore _array_element)
      (Utilities|Array|Clear _lastplaceplayers)
      (Utilities|Array|AppendArray _lastplaceplayers (Utilities|Array|MakeArray (Utilities|Array|Get(acopy) (Variables|/Game/Minigame/Blueprints/BP_MinigameMode.BP_MinigameMode_C|GetPlayers (Variables|Default|GetGameModeRef)) _array_index)))
      (elif (== _array_element (LocalVariables|GetLastPlaceScore))
        (Utilities|Array|AppendArray (Variables|Default|GetLastPlacePlayers) (Utilities|Array|MakeArray (Utilities|Array|Get(acopy) (Variables|/Game/Minigame/Blueprints/BP_MinigameMode.BP_MinigameMode_C|GetPlayers (Variables|Default|GetGameModeRef)) _array_index)))))))

(fn DetermineNextMinigame
  (bind _doorswitheligibleplayers (LocalVariables|GetDoorsWithEligiblePlayers))
  (bind _output (Utilities|Array|Get(acopy) _doorswitheligibleplayers))
  ;[1 1 1] Loops to see if any doors have last place players stood at them, if so add to array of doors to randomly decide which minigame is next
  (for _array_element (Variables|Default|GetHubDoors)
    (if (> (Utilities|Array|Length (Variables|/Game/Minigame/Blueprints/Minigames/Hub/BP_HubDoor.BP_HubDoor_C|GetEligiblePlayersNearby _array_element)) 0)
      (Utilities|Array|AppendArray (LocalVariables|GetDoorsWithEligiblePlayers) (Utilities|Array|MakeArray _array_element))))
  ;[1 1 1] Determine if any doors are being stood in front of by last place players
  (if (> (Utilities|Array|Length (LocalVariables|GetDoorsWithEligiblePlayers)) 0)
    ;[1 1 1] Shuffles doors with last place players present and picks first one in new array
    (Utilities|Array|Shuffle _doorswitheligibleplayers)
    ;[1 1 1] Turns off lights of other doors that were not chosen
    (for _index (range 1 3)
      (Utilities|IsValid (Utilities|Array|Get(acopy) (LocalVariables|GetDoorsWithEligiblePlayers) _index)
        (:Is%20Valid
          (Default|TurnOffLight (Utilities|Array|Get(acopy) (LocalVariables|GetDoorsWithEligiblePlayers) _index)))))
    ;[1 1 1] Opens the picked random door and signals event to load minigame of indicated type
    (Default|OpenDoor _output)
    (Default|LoadNextMinigame (Variables|Default|GetGameModeRef) (Variables|/Game/Minigame/Blueprints/Minigames/Hub/BP_HubDoor.BP_HubDoor_C|GetNextMinigameType _output))
    (else
      ;[1 1 1] If no doors are chosen by a last place player, just select a door at random and additionally turn it's light on
      (bind _output_get (LocalVariables|SetShuffledDoors (Variables|Default|GetHubDoors)))
      (Utilities|Array|Shuffle _output_get)
      (Default|OpenDoor (Utilities|Array|Get(acopy) _output_get))
      (Default|TurnonLight (Utilities|Array|Get(acopy) _output_get))
      (Default|LoadNextMinigame (Variables|Default|GetGameModeRef) (Variables|/Game/Minigame/Blueprints/Minigames/Hub/BP_HubDoor.BP_HubDoor_C|GetNextMinigameType (Utilities|Array|Get(acopy) _output_get))))))

(fn AssignMinigamestoDoors
  (bind _output_get (LocalVariables|SetShuffleDoors (Variables|Default|GetHubDoors)))
  (Utilities|Array|Shuffle _output_get)
  (for _index (range 0 2)
    (switch int _index
      (:0
        (Default|SetMinigameType (Utilities|Array|Get(acopy) (LocalVariables|GetShuffleDoors) _index) "NewEnumerator0"))
      (:1
        (Default|SetMinigameType (Utilities|Array|Get(acopy) (LocalVariables|GetShuffleDoors) _index) "NewEnumerator1"))
      (:2
        (Default|SetMinigameType (Utilities|Array|Get(acopy) (LocalVariables|GetShuffleDoors) _index) "NewEnumerator2")))))