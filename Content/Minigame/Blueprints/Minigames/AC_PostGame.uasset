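; AC_PostGame is a post-game minigame component that determines which player won.
; GetWinningPlayer scans the PlayerScores array on the referenced game mode for the lowest score, so lower is better and the earliest entry wins a tie.
; It returns that score with a one-based player number, relying on the starting value of LowestScore as the threshold to beat.
; The event graph holds only disabled placeholder events.
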(event EventBeginPlay)

(event EventTick
  (params (DeltaSeconds :type Float%20%28single-precision%29)))

(fn GetWinningPlayer
  (for (_array_element _array_index) (Variables|/Game/Minigame/Blueprints/BP_MinigameMode.BP_MinigameMode_C|GetPlayerScores (Variables|Default|GetGameModeRef))
    (if (< _array_element (LocalVariables|GetLowestScore))
      (LocalVariables|SetLowestScore _array_element)
      (LocalVariables|SetLowestScoreIndex _array_index)))
  (return (+ (LocalVariables|GetLowestScoreIndex) 1) (LocalVariables|GetLowestScore)))