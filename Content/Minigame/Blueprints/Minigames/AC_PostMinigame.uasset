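; Post-minigame component that awards points to four players by rank and displays their scores.
; GetPointsFromRank maps rank to points, with higher rank numbers earning more, and AwardPoints adds them to the game mode's PlayerScores.
; DisplayNewScores writes the gained points and current PlayerScores into the minigame UI's added and old score texts.
; SetupPostMinigame takes the game mode reference and collects old-score text widgets.
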(event EventBeginPlay)

(event EventTick
  (params (DeltaSeconds :type Float%20%28single-precision%29)))

(fn DisplayNewScores
  (params (PrevGameRanks :type Array%20of%20Integers))
  (bind _gamemoderef (Variables|Default|GetGameModeRef))
  (bind _gamemoderef_2 (Variables|Default|GetGameModeRef))
  (bind _minigameuiref (Variables|/Game/Minigame/Blueprints/BP_MinigameMode.BP_MinigameMode_C|GetMinigameUIRef _gamemoderef_2))
  (bind _minigameuiref_2 (Variables|/Game/Minigame/Blueprints/BP_MinigameMode.BP_MinigameMode_C|GetMinigameUIRef _gamemoderef))
  (for (_array_element _array_index) PrevGameRanks
    (bind _points (CallFunction|GetPointsfromRank _array_element))
    (switch int _array_index
      (:0
        (Rendering|Components|TextRender|SetText (Variables|/Game/Minigame/Blueprints/WBP_MinigameUI.WBP_MinigameUI_C|GetP1AddedScoreText _minigameuiref_2) (Utilities|Text|ToText(String) (Utilities|String|Append "+" (Utilities|String|ToString(Integer) _points)))))
      (:1
        (Rendering|Components|TextRender|SetText (Variables|/Game/Minigame/Blueprints/WBP_MinigameUI.WBP_MinigameUI_C|GetP2AddedScoreText _minigameuiref_2) (Utilities|Text|ToText(String) (Utilities|String|Append "+" (Utilities|String|ToString(Integer) _points)))))
      (:2
        (Rendering|Components|TextRender|SetText (Variables|/Game/Minigame/Blueprints/WBP_MinigameUI.WBP_MinigameUI_C|GetP3AddedScoreText _minigameuiref_2) (Utilities|Text|ToText(String) (Utilities|String|Append "+" (Utilities|String|ToString(Integer) _points)))))
      (:3
        (Rendering|Components|TextRender|SetText (Variables|/Game/Minigame/Blueprints/WBP_MinigameUI.WBP_MinigameUI_C|GetP4AddedScoreText _minigameuiref_2) (Utilities|Text|ToText(String) (Utilities|String|Append "+" (Utilities|String|ToString(Integer) _points)))))))
  (for _index (range 0 3)
    (switch int _index
      (:0
        (Rendering|Components|TextRender|SetText (Variables|/Game/Minigame/Blueprints/WBP_MinigameUI.WBP_MinigameUI_C|GetP1OldScoreText _minigameuiref) (Utilities|Text|ToText(Integer) (Utilities|Array|Get(acopy) (Variables|/Game/Minigame/Blueprints/BP_MinigameMode.BP_MinigameMode_C|GetPlayerScores (Variables|Default|GetGameModeRef)) _index))))
      (:1
        (Rendering|Components|TextRender|SetText (Variables|/Game/Minigame/Blueprints/WBP_MinigameUI.WBP_MinigameUI_C|GetP2OldScoreText _minigameuiref) (Utilities|Text|ToText(Integer) (Utilities|Array|Get(acopy) (Variables|/Game/Minigame/Blueprints/BP_MinigameMode.BP_MinigameMode_C|GetPlayerScores (Variables|Default|GetGameModeRef)) _index))))
      (:2
        (Rendering|Components|TextRender|SetText (Variables|/Game/Minigame/Blueprints/WBP_MinigameUI.WBP_MinigameUI_C|GetP3OldScoreText _minigameuiref) (Utilities|Text|ToText(Integer) (Utilities|Array|Get(acopy) (Variables|/Game/Minigame/Blueprints/BP_MinigameMode.BP_MinigameMode_C|GetPlayerScores (Variables|Default|GetGameModeRef)) _index))))
      (:3
        (Rendering|Components|TextRender|SetText (Variables|/Game/Minigame/Blueprints/WBP_MinigameUI.WBP_MinigameUI_C|GetP4OldScoreText _minigameuiref) (Utilities|Text|ToText(Integer) (Utilities|Array|Get(acopy) (Variables|/Game/Minigame/Blueprints/BP_MinigameMode.BP_MinigameMode_C|GetPlayerScores (Variables|Default|GetGameModeRef)) _index)))))))

(fn SetupPostMinigame
  (params (GameModeRef :type BP%20Minigame%20Mode%20Object%20Reference))
  (bind _oldscoretexts (Variables|Default|GetOldScoreTexts))
  (Utilities|IsValid (Variables|Default|GetGameModeRef)
    (:Is%20Valid
      _)
    (:Is%20Not%20Valid
      (Variables|Default|SetGameModeRef GameModeRef)))
  (if (< (Utilities|Array|Length (Variables|Default|GetOldScoreTexts)) 1)
    (bind _counter (Utilities|FlowControl|DoN 4)
      (:Exit
        (switch int _counter
          (:1
            (Utilities|Array|AppendArray _oldscoretexts (Utilities|Array|MakeArray (Variables|/Game/Minigame/Blueprints/WBP_MinigameUI.WBP_MinigameUI_C|GetP1OldScoreText (Variables|/Game/Minigame/Blueprints/BP_MinigameMode.BP_MinigameMode_C|GetMinigameUIRef (Variables|Default|GetGameModeRef))))))
          (:2
            (Utilities|Array|AppendArray _oldscoretexts (Utilities|Array|MakeArray (Variables|/Game/Minigame/Blueprints/WBP_MinigameUI.WBP_MinigameUI_C|GetP2OldScoreText (Variables|/Game/Minigame/Blueprints/BP_MinigameMode.BP_MinigameMode_C|GetMinigameUIRef (Variables|Default|GetGameModeRef))))))
          (:3
            (Utilities|Array|AppendArray _oldscoretexts (Utilities|Array|MakeArray (Variables|/Game/Minigame/Blueprints/WBP_MinigameUI.WBP_MinigameUI_C|GetP3OldScoreText (Variables|/Game/Minigame/Blueprints/BP_MinigameMode.BP_MinigameMode_C|GetMinigameUIRef (Variables|Default|GetGameModeRef))))))
          (:4
            (Utilities|Array|AppendArray _oldscoretexts (Utilities|Array|MakeArray (Variables|/Game/Minigame/Blueprints/WBP_MinigameUI.WBP_MinigameUI_C|GetP4OldScoreText (Variables|/Game/Minigame/Blueprints/BP_MinigameMode.BP_MinigameMode_C|GetMinigameUIRef (Variables|Default|GetGameModeRef)))))))))))

(fn GetPointsfromRank
  (params (Rank :type Integer))
  (switch int Rank
    (:1
      (return 0))
    (:2
      (return 2))
    (:3
      (return 3))
    (:4
      (return 5))))

(fn AwardPoints
  (params (MinigameRanks :type Array%20of%20Integers))
  (LocalVariables|SetPlayer%20Ranks MinigameRanks)
  (for (_array_element _array_index) (Variables|/Game/Minigame/Blueprints/BP_MinigameMode.BP_MinigameMode_C|GetPlayerScores (Variables|Default|GetGameModeRef))
    (bind _points (CallFunction|GetPointsfromRank (Utilities|Array|Get(acopy) (LocalVariables|GetPlayer%20Ranks) _array_index)))
    (Utilities|Array|SetArrayElem (Variables|/Game/Minigame/Blueprints/BP_MinigameMode.BP_MinigameMode_C|GetPlayerScores (Variables|Default|GetGameModeRef)) _array_index (+ _array_element _points))))