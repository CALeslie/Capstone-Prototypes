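; Game mode for the hub between minigame rounds, where last-place (highest-score) players influence which minigame comes next.
; BeginPlay advances the round or ends the game, shuffles door types and player spawns, fills scoreboards and fades in.
; When the countdown expires, it opens a random door among those with eligible players nearby, or any door otherwise.
; It then fades out to load the level; only Hiding is implemented.
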(event Custom|ChoosingFinished_
  (CallFunction|ToggleAllPlayersControl false)
  (Variables|Default|SetHubStatus "NewEnumerator1")
  (bind _timeropacity (Timeline|ChoosingFinishedAnim_ PlayFromStart)
    (:Update
      (CallFunction|SetTimerOpacity _timeropacity))
    (:Finished
      (CallFunction|DetermineNextMinigame))))

(event Custom|LoadNextMinigame_
  (params (Type :type EN_HubDoorType%20Enum :default "NewEnumerator0"))
  (Utilities|FlowControl|Delay 1.0)
  (bind _fadeopacity (Timeline|HubFadeOut_ PlayFromStart)
    (:Update
      (Default|SetBlackFadeOpacity (Variables|UI|GetBlackFade) _fadeopacity))
    (:Finished
      (switch Utilities|FlowControl|Switch|SwitchonEN_HubDoorType Type
        (:NewEnumerator0
          _)
        (:NewEnumerator1
          (Development|PrintString "Not Implemented Yet!" :!label _label))
        (:NewEnumerator2
          (goto _label)))
      (Game|OpenLevel(byObjectReference) "/Game/Minigame/Maps/HideNSneakLevel.HideNSneakLevel"))))

(event EventBeginPlay
  (|CallParentFunction)
  (bind _asbp_game_instance (Utilities|Casting|CastToBP_GameInstance (Game|GetGameInstance)))
  (bind _output_get (Variables|Default|SetGameInstance _asbp_game_instance))
  (Math|Integer|IncrementInt (Variables|/Game/Minigame/Blueprints/BP_GameInstance.BP_GameInstance_C|GetCurrRound _output_get)
    (:%20%20
      (if (<= (Variables|/Game/Minigame/Blueprints/BP_GameInstance.BP_GameInstance_C|GetCurrRound _output_get) (Variables|Default|GetNumRounds))
        (Variables|/Game/Minigame/Blueprints/BP_GameInstance.BP_GameInstance_C|SetCurrGameState (Variables|Default|GetGameInstance) "NewEnumerator1")
        (bind _returnvalue (UserInterface|CreateWidget "/Game/Minigame/Blueprints/Widgets/WBP_Timer.WBP_Timer_C"))
        (UserInterface|Viewport|AddtoViewport _returnvalue 0)
        (CallFunction|SetTimerRef _returnvalue)
        (CallFunction|SetTimerOpacity 1.0)
        (bind _returnvalue_2 (UserInterface|CreateWidget "/Game/Minigame/Blueprints/Widgets/WBP_BlackFade.WBP_BlackFade_C"))
        (bind _output_get_2 (Variables|UI|SetBlackFade _returnvalue_2))
        (UserInterface|Viewport|AddtoViewport _output_get_2 0)
        (Default|SetBlackFadeOpacity _output_get_2 1.0)
        (CallFunction|HubSetup)
        (CallFunction|SetUpPlayers)
        (Variables|Default|SetMinigameTimer (Variables|Default|GetTimeToChoose))
        (Utilities|FlowControl|Delay 0.2)
        (Default|RegisterPlayerActors (Variables|Default|GetDevMenuRef))
        (CallFunction|SetTimerText)
        (CallFunction|HandleGameSave)
        (CallFunction|SetPlayersVisibilities true)
        (bind _fadeopacity (Timeline|HubFadeIn_ PlayFromStart)
          (:Update
            (Default|SetBlackFadeOpacity (Variables|UI|GetBlackFade) _fadeopacity))
          (:Finished
            (CallFunction|ToggleAllPlayersControl true)))
        (else
          (CallFunction|EndOfGame))))))

(event EventTick
  (params (DeltaSeconds :type Float%20%28single-precision%29))
  (if (Utilities|Enum|Equal(Enum) (Variables|Default|GetHubStatus) "NewEnumerator0")
    (CallFunction|UpdateTimer DeltaSeconds)
    (CallFunction|TimerCheck)))

(fn ConstructionScript
  (|CallParentFunction))

(fn SetUpPlayers
  (CallFunction|SpawnPlayers)
  (bind _outactors (Actor|GetAllActorsOfClass "/Game/Minigame/Blueprints/BP_MinigameCharacter.BP_MinigameCharacter_C"))
  (Variables|Default|SetPlayers_ _outactors)
  (bind _outactors_2 (Actor|GetAllActorsOfClass "/Game/Minigame/Blueprints/BP_PlayerStart.BP_PlayerStart_C"))
  (bind _output_get (LocalVariables|SetPlayerStarts _outactors_2))
  (Utilities|Array|Shuffle _output_get)
  (for (_array_element _array_index) (LocalVariables|GetPlayerStarts)
    (Transformation|SetActorLocationAndRotation (Utilities|Array|Get(acopy) (Variables|Default|GetPlayers_) _array_index) (Math|Vector|MakeVector (.x (Transformation|GetActorLocation _array_element)) (.y (Transformation|GetActorLocation _array_element)) (+ (.z (Transformation|GetActorLocation _array_element)) 30.62)) (Transformation|GetActorRotation _array_element) false true)
    (Default|TogglePlayerVisibility (Utilities|Array|Get(acopy) (Variables|Default|GetPlayers_) _array_index) true)
    (Default|RefreshCameraRef (Utilities|Array|Get(acopy) (Variables|Default|GetPlayers_) _array_index))))

(fn SetLastPlacePlayers
  (bind _lastplaceplayers (Variables|Default|GetLastPlacePlayers))
  (bind _asbp_game_instance (Utilities|Casting|CastToBP_GameInstance (Game|GetGameInstance)))
  (for (_array_element _array_index) (Variables|/Game/Minigame/Blueprints/BP_GameInstance.BP_GameInstance_C|GetPlayerScores _asbp_game_instance)
    (if (> _array_element (LocalVariables|GetLastPlaceScore))
      (LocalVariables|SetLastPlaceScore _array_element)
      (Utilities|Array|Clear _lastplaceplayers)
      (Utilities|Array|AppendArray _lastplaceplayers (Utilities|Array|MakeArray (Utilities|Array|Get(acopy) (Variables|Default|GetPlayers_) _array_index)))
      (elif (== _array_element (LocalVariables|GetLastPlaceScore))
        (Utilities|Array|AppendArray (Variables|Default|GetLastPlacePlayers) (Utilities|Array|MakeArray (Utilities|Array|Get(acopy) (Variables|Default|GetPlayers_) _array_index)))))))

(fn DetermineNextMinigame
  (bind _doorswitheligibleplayers (LocalVariables|GetDoorsWithEligiblePlayers))
  (bind _output (Utilities|Array|Get(acopy) _doorswitheligibleplayers))
  ;[1 1 1] Loops to see if any doors have last place players stood at them, if so add to array of doors to randomly decide which minigame is next
  (for _array_element (Variables|Default|GetHubDoors)
    (if (> (Utilities|Array|Length (Variables|/Game/Minigame/Blueprints/Minigames/Hub/BP_HubDoor.BP_HubDoor_C|GetEligiblePlayersNearby _array_element)) 0)
      (Utilities|Array|AppendArray (LocalVariables|GetDoorsWithEligiblePlayers) (Utilities|Array|MakeArray _array_element))))
  ;[1 1 1] Determine if any doors are being stood in front of by last place players
  (if (> (Utilities|Array|Length (LocalVariables|GetDoorsWithEligiblePlayers)) 0)
    ;[1 1 1] Shuffles doors with last place players present and picks first one in new array
    (Utilities|Array|Shuffle _doorswitheligibleplayers)
    ;[1 1 1] Turns off lights of other doors that were not chosen
    (for _index (range 1 3)
      (Utilities|IsValid (Utilities|Array|Get(acopy) (LocalVariables|GetDoorsWithEligiblePlayers) _index)
        (:Is%20Valid
          (Default|TurnOffLight (Utilities|Array|Get(acopy) (LocalVariables|GetDoorsWithEligiblePlayers) _index)))))
    ;[1 1 1] Opens the picked random door and signals event to load minigame of indicated type
    (Default|OpenDoor _output)
    (CallFunction|LoadNextMinigame (Variables|/Game/Minigame/Blueprints/Minigames/Hub/BP_HubDoor.BP_HubDoor_C|GetNextMinigameType _output))
    (else
      ;[1 1 1] If no doors are chosen by a last place player, just select a door at random and additionally turn it's light on
      (bind _output_get (LocalVariables|SetShuffledDoors (Variables|Default|GetHubDoors)))
      (Utilities|Array|Shuffle _output_get)
      (Default|OpenDoor (Utilities|Array|Get(acopy) _output_get))
      (Default|TurnonLight (Utilities|Array|Get(acopy) _output_get))
      (CallFunction|LoadNextMinigame (Variables|/Game/Minigame/Blueprints/Minigames/Hub/BP_HubDoor.BP_HubDoor_C|GetNextMinigameType (Utilities|Array|Get(acopy) _output_get))))))

(fn AssignMinigamestoDoors
  (bind _output_get (LocalVariables|SetShuffleDoors (Variables|Default|GetHubDoors)))
  (Utilities|Array|Shuffle _output_get)
  (for _index (range 0 2)
    (switch int _index
      (:0
        (Default|SetMinigameType (Utilities|Array|Get(acopy) (LocalVariables|GetShuffleDoors) _index) "NewEnumerator0"))
      (:1
        (Default|SetMinigameType (Utilities|Array|Get(acopy) (LocalVariables|GetShuffleDoors) _index) "NewEnumerator1"))
      (:2
        (Default|SetMinigameType (Utilities|Array|Get(acopy) (LocalVariables|GetShuffleDoors) _index) "NewEnumerator2")))))

(fn HubSetup
  (CallFunction|SetLastPlacePlayers)
  (bind _outactors (Actor|GetAllActorsOfClass "/Game/Minigame/Blueprints/Minigames/Hub/BP_HubDoor.BP_HubDoor_C"))
  (Variables|Default|SetHubDoors _outactors)
  (bind _outactors_2 (Actor|GetAllActorsOfClass "/Game/Minigame/Blueprints/BP_SpotLightControl.BP_SpotLightControl_C"))
  (Variables|Default|SetHubDoorLights _outactors_2)
  (CallFunction|AssignMinigamestoDoors)
  (Variables|Default|SetHubStatus "NewEnumerator0")
  (bind _outactors_3 (Actor|GetAllActorsOfClass "/Game/Minigame/Blueprints/Minigames/Hub/BP_ScoreBoard.BP_ScoreBoard_C"))
  (bind _output_get (Variables|Default|SetScoreboards _outactors_3))
  (bind _asbp_game_instance (Utilities|Casting|CastToBP_GameInstance (Game|GetGameInstance)))
  (for (_array_element _array_index) (Variables|/Game/Minigame/Blueprints/BP_GameInstance.BP_GameInstance_C|GetPlayerScores _asbp_game_instance)
    (Default|SetPlayerScore (Utilities|Array|Get(acopy) _output_get) _array_index _array_element)
    (Default|SetPlayerScore (Utilities|Array|Get(acopy) _output_get 1) _array_index _array_element)))

(fn TimerCheck
  (if (<= (Variables|Default|GetMinigameTimer) 0.1)
    (CallFunction|ChoosingFinished)))