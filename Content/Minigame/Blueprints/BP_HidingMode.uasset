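; Game mode for a multiplayer hide-and-seek minigame where an enemy eliminates players each round until one or none remain.
; Setup spawns players at shuffled starts, then timelines drive fades, countdown, door and elimination cutscenes.
; A status enum gates player control and the tick-driven hiding timer, whose expiry triggers elimination.
; Surviving rounds reset hiding spots and players; a winner's finish saves ranks to the GameInstance and opens score review.
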(event Custom|CountdownFinished_
  (CallFunction|UpdateMinigameStatus "NewEnumerator3")
  (bind _timeropacity (Timeline|EliminatePlayer_ PlayFromStart)
    (:Update
      (CallFunction|SetTimerOpacity _timeropacity) ; Fades out counter while playing elimination cutscene
    )
    (:ElimPlayerEvent
      (CallFunction|EliminatePlayers))
    (:OpenDoorEvent
      (CallFunction|OpenDoor))))

(event Custom|EliminationFinished_
  ;[1 1 1] Executes after a round of eliminations is completed, checks if players are still left and if the game should be over or not, resets for another round of hiding if not
  (bind _result (CallFunction|CheckPlayersLeft))
  (if _result
    (bind _timeropacity (Timeline|FinishElimination_ PlayFromStart)
      (:Update
        (if (not (Utilities|Enum|Equal(Enum) (Variables|Default|GetMinigameStatus) "NewEnumerator2"))
          (CallFunction|SetTimerOpacity _timeropacity) ; Fades out counter while playing elimination cutscene
        ))
      (:Finished
        (CallFunction|UpdateHidingSpots)
        (bind _result_2 (CallFunction|CheckPlayersLeft))
        (if _result_2
          (CallFunction|UpdateMinigameStatus "NewEnumerator1")
          (else
            ;[1 1 1] This whole section handles wrapping up the end of the minigame
            (CallFunction|UpdateMinigameStatus "NewEnumerator2")
            (CallFunction|ToggleAllPlayersControl false)
            (for _array_element (Variables|Default|GetPlayers)
              (if (not (Variables|/Game/Minigame/Blueprints/BP_MinigameCharacter.BP_MinigameCharacter_C|GetCaught _array_element))
                (bind _output_get (Variables|Default|SetLastPlayer _array_element))
                (Utilities|Array|SetArrayElem (Variables|Default|GetPlayerRanks) (Variables|/Game/Minigame/Blueprints/BP_MinigameCharacter.BP_MinigameCharacter_C|GetPlayerID _output_get) 1)))
            (Utilities|IsValid (Variables|Default|GetLastPlayer)
              (:Is%20Valid
                (CallFunction|SetCountdownText (Utilities|String|Append "Finished! P" (Utilities|String|ToString(Integer) (Variables|/Game/Minigame/Blueprints/BP_MinigameCharacter.BP_MinigameCharacter_C|GetPlayerID (Variables|Default|GetLastPlayer))) " won"))
                (bind _fadealpha (Timeline|FinishedTimeline_ PlayFromStart)
                  (:Update
                    (CallFunction|SetCountdownOpacity _fadealpha))
                  (:Finished
                    (Utilities|FlowControl|Delay 3.0)
                    (bind _opacity (Timeline|MinigameFadeOut PlayFromStart)
                      (:Update
                        (CallFunction|SetFadeOpacity _opacity))
                      (:Finished
                        (bind _opacity_2 (Timeline|FadeOutCountdown PlayFromStart)
                          (:Update
                            (CallFunction|SetCountdownOpacity _opacity_2))
                          (:Finished
                            (CallFunction|SetPlayersVisibilities false)
                            (bind _asbp_game_instance (Utilities|Casting|CastToBP_GameInstance (Game|GetGameInstance)))
                            (Variables|/Game/Minigame/Blueprints/BP_GameInstance.BP_GameInstance_C|SetPrevMinigameRanks _asbp_game_instance (Variables|Default|GetPlayerRanks))
                            (Game|OpenLevel(byObjectReference) "/Game/Minigame/Maps/ScoreReviewLevel.ScoreReviewLevel"))))))))
              (:Is%20Not%20Valid
                (CallFunction|SetCountdownText "Finished! No one won")
                (Timeline|FinishedTimeline_ PlayFromStart))))))
      (:CloseDoorEvent
        (Default|EventCloseDoor (Variables|Default|GetEnemyDoor))
        (Variables|Default|SetMinigameTimer (Variables|Default|GetTimeToHide))
        (CallFunction|SetTimerText)
        (CallFunction|ReshowPlayers)))
    (else
      (CallFunction|UpdateMinigameStatus "NewEnumerator2")
      (Timeline|FinishElimination_ PlayFromStart))))

(event EventBeginPlay
  (|CallParentFunction)
  (bind _asbp_game_instance (Utilities|Casting|CastToBP_GameInstance (Game|GetGameInstance)))
  (Variables|Default|SetGameInstance _asbp_game_instance)
  (CallFunction|ChangeGameState "NewEnumerator2")
  (CallFunction|MinigameSetup)
  (CallFunction|SetCountdownText "3")
  (CallFunction|SetupEnemyandPlayers)
  (Utilities|FlowControl|Delay 0.25)
  (bind _opacity (Timeline|FadeInMinigame PlayFromStart)
    (:Update
      (CallFunction|SetFadeOpacity _opacity))
    (:Finished
      (bind _fadealpha (Timeline|CountdownTimeline_ PlayFromStart)
        (:Update
          (CallFunction|SetCountdownOpacity _fadealpha))
        (:ChangeText
          (CallFunction|TickCountdownStep))
        (:GivePlayerControl
          (CallFunction|ToggleAllPlayersControl true)
          (CallFunction|UpdateMinigameStatus "NewEnumerator1"))))))

(event EventTick
  (params (DeltaSeconds :type Float%20%28single-precision%29))
  (if (Utilities|Enum|Equal(Enum) (Variables|Default|GetMinigameStatus) "NewEnumerator1")
    (CallFunction|UpdateTimer DeltaSeconds)
    (CallFunction|TimerCheck)))

(fn ConstructionScript
  (|CallParentFunction))

(fn MinigameSetup
  (bind _timetohide (Variables|Default|GetTimeToHide))
  (Variables|Default|SetMinigameStatus "NewEnumerator0")
  (CallFunction|CreateTimerWidget)
  (CallFunction|CreateFadeWidget)
  (CallFunction|CreateCountdownWidget)
  (bind _returnvalue (UserInterface|CreateWidget "/Game/Minigame/Blueprints/Widgets/WBP_InteractPrompts.WBP_InteractPrompts_C"))
  (bind _output_get (LocalVariables|SetInteractUi _returnvalue))
  (UserInterface|Viewport|AddtoViewport _output_get 0)
  (bind _returnvalue_2 (Actor|GetActorOfClass "/Game/Minigame/Blueprints/Minigames/Hiding/BP_Hide_Door.BP_Hide_Door_C"))
  (Variables|Default|SetEnemyDoor _returnvalue_2)
  (bind _outactors (Actor|GetAllActorsOfClass "/Game/Minigame/Blueprints/Minigames/Hiding/BP_HidingSpot.BP_HidingSpot_C"))
  (Variables|Default|SetHidingSpots _outactors)
  (Variables|Default|SetCaughtPlayers (Utilities|Array|MakeArray 0))
  (bind _outactors_2 (Actor|GetAllActorsOfClass "/Game/Minigame/Blueprints/Minigames/Hiding/BP_EnemyController.BP_EnemyController_C"))
  (bind _output_get_2 (Variables|Default|SetEnemy (Utilities|Array|Get(acopy) _outactors_2)))
  (Variables|/Game/Minigame/Blueprints/Minigames/Hiding/BP_EnemyController.BP_EnemyController_C|SetMinigameModeRef _output_get_2 self)
  (Variables|Default|SetMinigameTimer _timetohide)
  (CallFunction|SetTimerText)
  (Variables|Default|SetMinigameTimer (+ _timetohide 1.0))
  (CallFunction|SetTimerOpacity 1.0)
  (CallFunction|SetCountdownOpacity 0.0))

(fn UpdateMinigameStatus
  (params (New%20Status :type EN_HidingMinigameStatus%20Enum :default "NewEnumerator0"))
  (bind _output_get (Variables|Default|SetMinigameStatus New%20Status))
  (switch Utilities|FlowControl|Switch|SwitchonEN_HidingMinigameStatus _output_get
    (:NewEnumerator0
      (CallFunction|ToggleAllPlayersControl false :!label _label))
    (:NewEnumerator1
      (CallFunction|ToggleAllPlayersControl true))
    (:NewEnumerator3
      (goto _label))
    (:NewEnumerator2
      (goto _label))))

(fn EliminatePlayers
  (bind _enemy (Variables|Default|GetEnemy))
  (for _array_element (Variables|Default|GetPlayers)
    (if (not (Variables|/Game/Minigame/Blueprints/BP_MinigameCharacter.BP_MinigameCharacter_C|GetCaught _array_element))
      (if (not (Variables|/Game/Minigame/Blueprints/BP_MinigameCharacter.BP_MinigameCharacter_C|GetHidden _array_element))
        (LocalVariables|SetPlayersNotHidden true))))
  (if (LocalVariables|GetPlayersNotHidden)
    (Default|EliminatePlayers _enemy)
    (else
      (Default|EliminatePlayer _enemy))))

(fn OpenDoor
  (Default|EventOpenDoor (Variables|Default|GetEnemyDoor)))

(fn SetupEnemyandPlayers
  (CallFunction|SpawnPlayers)
  (Default|SetupEnemy (Variables|Default|GetEnemy) (Variables|Default|GetPlayers))
  (bind _outactors (Actor|GetAllActorsOfClass "/Game/Minigame/Blueprints/BP_PlayerStart.BP_PlayerStart_C"))
  (bind _output_get (LocalVariables|SetPlayerStarts _outactors))
  (Utilities|Array|Shuffle _output_get)
  (for (_array_element _array_index) (LocalVariables|GetPlayerStarts)
    (Transformation|SetActorLocationAndRotation (Utilities|Array|Get(acopy) (Variables|Default|GetPlayers) _array_index) (Math|Vector|MakeVector (.x (Transformation|GetActorLocation _array_element)) (.y (Transformation|GetActorLocation _array_element)) (+ (.z (Transformation|GetActorLocation _array_element)) 30.62)) (Transformation|GetActorRotation _array_element) false true)
    (Default|TogglePlayerVisibility (Utilities|Array|Get(acopy) (Variables|Default|GetPlayers) _array_index) true)))

(fn ReshowPlayer
  (params (PlayerRef :type BP%20Minigame%20Character%20Object%20Reference))
  (bind _output_get (LocalVariables|SetPlayer PlayerRef))
  (Transformation|SetActorRotation _output_get (Math|Rotator|MakeRotator 0.0 0.0 (+ (.yaw (Transformation|GetActorRotation (LocalVariables|GetPlayer))) 1.8e+02)))
  (Default|TogglePlayerVisibility (LocalVariables|GetPlayer) true)
  (if (Variables|/Game/Minigame/Blueprints/BP_MinigameCharacter.BP_MinigameCharacter_C|GetCaught (LocalVariables|GetPlayer))
    _
    (else
      (Variables|/Game/Minigame/Blueprints/BP_MinigameCharacter.BP_MinigameCharacter_C|SetHidden (LocalVariables|GetPlayer) false)
      (Variables|/Game/Minigame/Blueprints/BP_MinigameCharacter.BP_MinigameCharacter_C|SetControlEnabled (LocalVariables|GetPlayer) true)))
  (Default|PlayOpenAnim (Variables|/Game/Minigame/Blueprints/BP_MinigameCharacter.BP_MinigameCharacter_C|GetHidingSpotRef (LocalVariables|GetPlayer))))

(fn ReshowPlayers
  (for _array_element (Variables|Default|GetPlayers)
    (if (not (Variables|/Game/Minigame/Blueprints/BP_MinigameCharacter.BP_MinigameCharacter_C|GetCaught _array_element))
      (CallFunction|ReshowPlayer _array_element)))
  (Math|Integer|IncrementInt (Variables|Default|GetMinigameRounds)))

(fn CheckPlayersLeft
  (for _array_element (Variables|Default|GetPlayers)
    (if (not (Variables|/Game/Minigame/Blueprints/BP_MinigameCharacter.BP_MinigameCharacter_C|GetCaught _array_element))
      (Math|Integer|IncrementInt (LocalVariables|GetNumPlayersLeft))))
  (return (> (LocalVariables|GetNumPlayersLeft) 1)))

(fn UpdateHidingSpots
  (for _array_element (Variables|Default|GetHidingSpots)
    (Variables|/Game/Minigame/Blueprints/Minigames/Hiding/BP_HidingSpot.BP_HidingSpot_C|SetUsed _array_element false)))

(fn CatchPlayer
  (params (Player :type BP%20Minigame%20Character%20Object%20Reference))
  (bind _playerid (Variables|/Game/Minigame/Blueprints/BP_MinigameCharacter.BP_MinigameCharacter_C|GetPlayerID Player))
  (bind _playerranks (Variables|Default|GetPlayerRanks))
  (Default|PlayerCaught Player)
  (Utilities|Array|AppendArray (Variables|Default|GetCaughtPlayers) (Utilities|Array|MakeArray Player))
  (Utilities|Array|SetArrayElem _playerranks _playerid (+ (Utilities|Array|Get(acopy) _playerranks _playerid) (Variables|Default|GetMinigameRounds))))

(fn TimerCheck
  (if (<= (Variables|Default|GetMinigameTimer) 0.1)
    (CallFunction|CountdownFinished)))