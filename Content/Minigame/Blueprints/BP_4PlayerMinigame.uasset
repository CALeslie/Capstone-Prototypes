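; Game mode for a local multiplayer hide-and-sneak minigame where players hide before a timer expires and an enemy eliminates them.
; Sets up UI and save settings, spawns players at shuffled PlayerStarts, then runs a countdown.
; A status enum gates the Tick timer and player control, while timeline event tracks sequence fades, door and eliminations.
; Rounds repeat until under two players remain; a winner triggers a level reload.
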(event Custom|Event%20Give%20Player%20Control
  ;[1 1 1] Handles minigame setup all the way to the point of the minigame being in progress
  (CallFunction|UpdateMinigameStatus "NewEnumerator1"))

(event EventBeginPlay
  ;[1 1 1] Handles minigame setup all the way to the point of the minigame being in progress
  (CallFunction|MinigameSetup)
  (CallFunction|HandleGameSave)
  (bind _opacity (Timeline|BlackFadeOut PlayFromStart)
    (:Update
      (Default|SetBlackFadeOpacity (Variables|Default|GetMinigameUIRef) _opacity))
    (:SpawnPlayersEvent
      (CallFunction|SpawnPlayers)
      (Default|SetupEnemy (Variables|Default|GetEnemy) (Variables|Default|GetPlayers))
      (CallFunction|EventStartCountdown) ; This event goes to MinigameCountdownGraph, resumes at Event Give Player Control below when finished
    )))

(event EventTick
  (params (DeltaSeconds :type Float%20%28single-precision%29))
  (CallFunction|UpdateTimer DeltaSeconds)
  (CallFunction|TimerCheck))

(event EventHandleStartingNewPlayer
  (params (NewPlayer :type Player%20Controller%20Object%20Reference)))

(event EventPostLogin
  (params (NewPlayer :type Player%20Controller%20Object%20Reference))
  (Actor|DestroyActor NewPlayer))

(event Custom|Event%20Start%20Countdown
  ;[1 1 1] Executes at the beginning of the game to facilitate the countdown timer
  (bind _fadealpha (Timeline|CountdownTimeline PlayFromStart)
    (:Update
      (CallFunction|SetCountdownOpacity _fadealpha))
    (:ChangeText
      (CallFunction|TickCountdownStep))
    (:GivePlayerControl
      (CallFunction|TogglePlayerControl true)
      (Variables|Default|SetMinigameStatus "NewEnumerator1"))))

(event Custom|Event%20Countdown%20Finished
  ;[1 1 1] Executes everytime the ingame timer reaches 0, handles eliminating players
  (CallFunction|UpdateMinigameStatus "NewEnumerator3")
  (bind _timeropacity (Timeline|EliminatePlayer PlayFromStart)
    (:Update
      (CallFunction|SetTimerOpacity _timeropacity) ; Fades out counter while playing elimination cutscene
    )
    (:ElimPlayerEvent
      (CallFunction|EliminatePlayers))
    (:OpenDoorEvent
      (Default|EventOpenDoor (Variables|Default|GetMonsterDoor)))))

(event Custom|EliminationFinished
  ;[1 1 1] Executes after a round of eliminations is completed, checks if players are still left and if the game should be over or not, resets for another round of hiding if not
  (bind _result (CallFunction|CheckPlayersLeft)) ; Returns true if 2 or more players are still alive
  (if _result
    (bind _timeropacity (Timeline|FinishElimination PlayFromStart)
      (:Update
        (if (not (Utilities|Enum|Equal(Enum) (Variables|Default|GetMinigameStatus) "NewEnumerator2"))
          (CallFunction|SetTimerOpacity _timeropacity) ; Fades out counter while playing elimination cutscene
        ))
      (:Finished
        (CallFunction|UpdateHidingSpots)
        (bind _result_2 (CallFunction|CheckPlayersLeft)) ; Returns true if 2 or more players are still alive
        (if _result_2
          (CallFunction|UpdateMinigameStatus "NewEnumerator1")
          (else
            ;[1 1 1] This whole section handles wrapping up the end of the minigame
            (CallFunction|UpdateMinigameStatus "NewEnumerator2")
            (CallFunction|TogglePlayerControl false)
            (for _array_element (Variables|Default|GetPlayers)
              (if (not (Variables|/Game/Minigame/Blueprints/BP_MinigameCharacter.BP_MinigameCharacter_C|GetCaught _array_element))
                (Variables|Default|SetLastPlayer _array_element)))
            (Utilities|IsValid (Variables|Default|GetLastPlayer)
              (:Is%20Valid
                (CallFunction|SetCountdownText (Utilities|String|Append "Finished! P" (Utilities|String|ToString(Integer) (+ (Variables|/Game/Minigame/Blueprints/BP_MinigameCharacter.BP_MinigameCharacter_C|GetPlayerID (Variables|Default|GetLastPlayer)) 1)) " won"))
                (bind _fadealpha (Timeline|FinishedTimeline PlayFromStart)
                  (:Update
                    (CallFunction|SetCountdownOpacity _fadealpha))
                  (:Finished
                    (Utilities|FlowControl|Delay 3.0)
                    (bind _opacity (Timeline|BlackFadeIn PlayFromStart)
                      (:Update
                        (Default|SetBlackFadeOpacity (Variables|Default|GetMinigameUIRef) _opacity))
                      (:Finished
                        (Game|OpenLevel(byName) "HideNSneakLevel")
                        (for (_array_element_2 _array_index) (Variables|Default|GetPlayers)
                          (if (!= _array_index 0)
                            (bind _asplayer_controller (Utilities|Casting|CastToPlayerController (Pawn|GetController _array_element_2)))
                            (Class|GameplayStatics|RemovePlayer _asplayer_controller true))))))))
              (:Is%20Not%20Valid
                (CallFunction|SetCountdownText "Finished! No one won")
                (Timeline|FinishedTimeline PlayFromStart))))))
      (:CloseDoorEvent
        (Default|EventCloseDoor (Variables|Default|GetMonsterDoor))
        (Variables|Default|SetMinigameTimer (Variables|Default|GetTimeToHide))
        (CallFunction|SetTimerText)
        (CallFunction|ReshowPlayers)))
    (else
      (Variables|Default|SetMinigameStatus "NewEnumerator2")
      (Timeline|FinishElimination PlayFromStart))))

(fn ConstructionScript)

(fn SpawnPlayers
  ;[1 1 1] Gathers all player spawns in a randomized array and iterates over them (randomizes spawn locations, allows for more than 4 spawns)
  (bind _outactors (Actor|GetAllActorsOfClass "/Script/Engine.PlayerStart"))
  (bind _output_get (LocalVariables|SetPlayerStarts _outactors))
  (Utilities|Array|Shuffle _output_get)
  (Variables|Default|SetDefaultPawnClass "/Game/Minigame/Blueprints/BP_MinigameCharacter.BP_MinigameCharacter_C")
  (for (_array_element _array_index) _output_get
    ;[1 1 1] Creates player controller, if valid spawns character pawn at player start entity and then possesses pawn with that controller
    (bind _returnvalue (Class|GameplayStatics|CreatePlayer _array_index))
    (if (Utilities|IsValid _returnvalue)
      (bind _returnvalue_2 (Game|SpawnActorfromClass "/Game/Minigame/Blueprints/BP_MinigameCharacter.BP_MinigameCharacter_C" (Transformation|GetActorTransform _array_element) "AlwaysSpawn" "MultiplyWithRoot" 0 0))
      (Pawn|Possess _returnvalue _returnvalue_2)
      (Actor|DestroyActor _array_element) ; Destroys player starts after using to ensure multiple players aren't spawned on same ones
    ))
  ;[1 1 1] Required to clean up default spawned controller
  (Class|GameModeBase|RestartPlayer (Game|GetPlayerController 0))
  (bind _foundwidgets (Widget|GetAllWidgetsOfClass "/Game/Minigame/Blueprints/WBP_MovementControls.WBP_MovementControls_C" true))
  (Default|RegisterPlayerActors (Utilities|Array|Get(acopy) _foundwidgets))
  (Variables|/Script/Engine.PlayerController|SetbShowMouseCursor (Game|GetPlayerController 0) true)
  (bind _outactors_2 (Actor|GetAllActorsOfClass "/Game/Minigame/Blueprints/BP_MinigameCharacter.BP_MinigameCharacter_C"))
  (bind _output_get_2 (Variables|Default|SetPlayers _outactors_2))
  (for (_array_element_2 _array_index_2) _output_get_2
    (Variables|/Game/Minigame/Blueprints/BP_MinigameCharacter.BP_MinigameCharacter_C|SetPlayerID _array_element_2 _array_index_2)))

(fn MinigameSetup
  (bind _timetohide (Variables|Default|GetTimeToHide))
  (bind _returnvalue (Actor|GetActorOfClass "/Game/Minigame/Blueprints/BP_Hide_Door.BP_Hide_Door_C"))
  (Variables|Default|SetMonsterDoor _returnvalue)
  (bind _returnvalue_2 (UserInterface|CreateWidget "/Game/Minigame/Blueprints/WBP_MovementControls.WBP_MovementControls_C"))
  (UserInterface|Viewport|AddtoViewport _returnvalue_2 0)
  (Variables|Default|SetMovementControlsRef _returnvalue_2)
  (bind _returnvalue_3 (UserInterface|CreateWidget "/Game/Minigame/Blueprints/WBP_MinigameUI.WBP_MinigameUI_C"))
  (UserInterface|Viewport|AddtoViewport _returnvalue_3 0)
  (Variables|Default|SetMinigameUIRef _returnvalue_3)
  (bind _outactors (Actor|GetAllActorsOfClass "/Game/Minigame/Blueprints/BP_HidingSpot.BP_HidingSpot_C"))
  (Variables|Default|SetHidingSpots _outactors)
  (bind _outactors_2 (Actor|GetAllActorsOfClass "/Game/Minigame/Blueprints/BP_EnemyController.BP_EnemyController_C"))
  (bind _output_get (Variables|Default|SetEnemy (Utilities|Array|Get(acopy) _outactors_2)))
  (Variables|/Game/Minigame/Blueprints/BP_EnemyController.BP_EnemyController_C|SetMinigameModeRef _output_get self)
  (Variables|Default|SetMinigameTimer _timetohide)
  (CallFunction|SetTimerText)
  (Variables|Default|SetMinigameTimer (+ _timetohide 1.0)))

(fn TimerCheck
  (if (Utilities|Enum|Equal(Enum) (Variables|Default|GetMinigameStatus) "NewEnumerator1")
    (if (<= (Variables|Default|GetMinigameTimer) 0.1)
      (CallFunction|EventCountdownFinished))))

(fn UpdateTimer
  (params (Delta%20Time :type Float%20%28double-precision%29))
  ;[1 1 1] Updates minigame timer internally once per frame, updates UI element once per second
  (if (Utilities|Enum|Equal(Enum) (Variables|Default|GetMinigameStatus) "NewEnumerator1")
    (Variables|Default|SetMinigameTimer (- (Variables|Default|GetMinigameTimer) Delta%20Time))
    (bind _output_get (Variables|Default|SetMinigameUpdateTimer (+ (Variables|Default|GetMinigameUpdateTimer) Delta%20Time)))
    (if (>= _output_get 1.0)
      (Default|SetTimerText (Variables|Default|GetMinigameUIRef) (Utilities|Text|ToText(Integer) (Math|Float|Floor (Variables|Default|GetMinigameTimer))))
      (Variables|Default|SetMinigameUpdateTimer 0.0))))

(fn TogglePlayerControl
  (params (PlayerControl :type Boolean))
  (bind _outactors (Actor|GetAllActorsOfClass "/Game/Minigame/Blueprints/BP_MinigameCharacter.BP_MinigameCharacter_C"))
  (for _array_element _outactors
    (Variables|/Game/Minigame/Blueprints/BP_MinigameCharacter.BP_MinigameCharacter_C|SetControlEnabled _array_element PlayerControl)))

(fn UpdateMinigameStatus
  (params (New%20Status :type EN_MinigameStatus%20Enum :default "NewEnumerator0"))
  (bind _output_get (Variables|Default|SetMinigameStatus New%20Status))
  (switch Utilities|FlowControl|Switch|SwitchonEN_MinigameStatus _output_get
    (:NewEnumerator1
      (CallFunction|TogglePlayerControl true))
    (:NewEnumerator3
      (CallFunction|TogglePlayerControl false))))

(fn UpdateHidingSpots
  (for _array_element (Variables|Default|GetHidingSpots)
    (Variables|/Game/Minigame/Blueprints/BP_HidingSpot.BP_HidingSpot_C|SetUsed _array_element false)))

(fn CheckPlayersLeft
  (for _array_element (Variables|Default|GetPlayers)
    (if (not (Variables|/Game/Minigame/Blueprints/BP_MinigameCharacter.BP_MinigameCharacter_C|GetCaught _array_element))
      (Math|Integer|IncrementInt (LocalVariables|GetNumPlayersLeft))))
  (return (> (LocalVariables|GetNumPlayersLeft) 1)))

(fn SetTimerOpacity
  (params (NewOpacity :type Float%20%28double-precision%29))
  (Default|SetTimerOpacity (Variables|Default|GetMinigameUIRef) NewOpacity))

(fn SetCountdownOpacity
  (params (NewOpacity :type Float%20%28double-precision%29))
  (Default|SetCountdownOpacity (Variables|Default|GetMinigameUIRef) NewOpacity))

(fn TickCountdownStep
  (bind _minigameuiref (Variables|Default|GetMinigameUIRef))
  (switch int (Variables|Default|GetCountdownStep)
    (:0
      (Default|SetCountdownText _minigameuiref "2"))
    (:1
      (Default|SetCountdownText _minigameuiref "1"))
    (:2
      (Default|SetCountdownText _minigameuiref "Start!")))
  (Math|Integer|IncrementInt (Variables|Default|GetCountdownStep)))

(fn EliminatePlayers
  (bind _enemy (Variables|Default|GetEnemy))
  (for _array_element (Variables|Default|GetPlayers)
    (if (not (Variables|/Game/Minigame/Blueprints/BP_MinigameCharacter.BP_MinigameCharacter_C|GetCaught _array_element))
      (if (not (Variables|/Game/Minigame/Blueprints/BP_MinigameCharacter.BP_MinigameCharacter_C|GetHidden _array_element))
        (LocalVariables|SetPlayersNotHidden true))))
  (if (LocalVariables|GetPlayersNotHidden)
    (Default|EliminatePlayers _enemy)
    (else
      (Default|EliminatePlayer _enemy))))

(fn SetTimerText
  (Default|SetTimerText (Variables|Default|GetMinigameUIRef) (Utilities|Text|ToText(Integer) (Math|Float|Floor (Variables|Default|GetMinigameTimer)))))

(fn ReshowPlayers
  (for _array_element (Variables|Default|GetPlayers)
    (if (not (Variables|/Game/Minigame/Blueprints/BP_MinigameCharacter.BP_MinigameCharacter_C|GetCaught _array_element))
      (Default|EventReshowPlayer _array_element))))

(fn SetCountdownText
  (params (NewText :type String))
  (Default|SetCountdownText (Variables|Default|GetMinigameUIRef) (Utilities|Text|ToText(String) NewText)))

(fn HandleGameSave
  (bind _returnvalue (SaveGame|LoadGamefromSlot "GameSettings"))
  (Utilities|IsValid _returnvalue
    (:Is%20Valid
      (bind _asbp_game_save (Utilities|Casting|CastToBP_GameSave _returnvalue))
      (bind _output_get (Variables|Default|SetGameSaveRef _asbp_game_save))
      (Default|LoadInstanceSettings (Variables|Default|GetMovementControlsRef) (Variables|/Game/Minigame/Blueprints/BP_GameSave.BP_GameSave_C|GetSavedPreset _output_get)))
    (:Is%20Not%20Valid
      (bind _returnvalue_2 (SaveGame|CreateSaveGameObject "/Game/Minigame/Blueprints/BP_GameSave.BP_GameSave_C"))
      (SaveGame|SaveGametoSlot _returnvalue_2 "GameSettings")))
  (return))