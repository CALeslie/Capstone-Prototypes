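; ConcussEffect is a Blueprint for a concussion visual effect in a minigame, built on three meshes with adjustable opacity.
; AssignDynamicMatInstance creates one dynamic instance of M_ConcussEffect, shares it across the three meshes and sets it to zero opacity.
; UpdateConcussOpacity drives the RenderOpacity parameter on that shared instance, changing all three meshes at once.
; BeginPlay and Tick are empty, and neither setup nor fading is triggered within the Blueprint itself.
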(event EventBeginPlay)

(event EventTick
  (params (DeltaSeconds :type Float%20%28single-precision%29)))

(fn UpdateConcussOpacity
  (params (Opacity :type Float%20%28double-precision%29))
  (Rendering|Material|SetScalarParameterValue (Variables|Default|GetConcussMat) "RenderOpacity" Opacity :!class /Script/Engine.MaterialInstanceDynamic))

(fn AssignDynamicMatInstance
  (bind _returnvalue (Rendering|Material|CreateDynamicMaterialInstance "/Game/Minigame/Materials/M_ConcussEffect.M_ConcussEffect" "None" "None" :!class /Script/Engine.KismetMaterialLibrary))
  (Variables|Default|SetConcussMat _returnvalue)
  (Rendering|Material|SetMaterial (Variables|Default|GetMesh1) 0 (Variables|Default|GetConcussMat))
  (Rendering|Material|SetMaterial (Variables|Default|GetMesh2) 0 (Variables|Default|GetConcussMat))
  (Rendering|Material|SetMaterial (Variables|Default|GetMesh3) 0 (Variables|Default|GetConcussMat))
  (CallFunction|UpdateConcussOpacity 0.0))