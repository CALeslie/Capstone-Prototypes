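; BP_HS_Closet is a minigame closet actor with two animated doors.
; PlayOpenAnim plays the OpenAnim timeline, which drives separate left and right yaw tracks into DoorLeft and DoorRight.
; PlayCloseAnim reverses the same timeline to close them.
; Door rotations are set in world space with zero pitch and roll, so the swing ignores the actor's own orientation.
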(event EventBeginPlay
  (|CallParentFunction) ; This node is disabled and will not be called.\nDrag off pins to build functionality.
)

(event Collision|EventActorBeginOverlap
  (params (OtherActor :type Actor%20Object%20Reference))
  (|CallParentFunction OtherActor) ; This node is disabled and will not be called.\nDrag off pins to build functionality.
)

(event EventTick
  (params (DeltaSeconds :type Float%20%28single-precision%29))
  (|CallParentFunction DeltaSeconds) ; This node is disabled and will not be called.\nDrag off pins to build functionality.
)

(event EventPlayOpenAnim
  (bind (_direction _ldoorrotation _rdoorrotation) (Timeline|OpenAnim Play)
    (:Update
      (Transformation|SetWorldRotation (Variables|Default|GetDoorLeft) (Math|Rotator|MakeRotator 0.0 0.0 _ldoorrotation) false false)
      (Transformation|SetWorldRotation (Variables|Default|GetDoorRight) (Math|Rotator|MakeRotator 0.0 0.0 _rdoorrotation) false false))))

(event EventPlayCloseAnim
  (bind (_direction _ldoorrotation _rdoorrotation) (Timeline|OpenAnim Reverse)
    (:Update
      (Transformation|SetWorldRotation (Variables|Default|GetDoorLeft) (Math|Rotator|MakeRotator 0.0 0.0 _ldoorrotation) false false)
      (Transformation|SetWorldRotation (Variables|Default|GetDoorRight) (Math|Rotator|MakeRotator 0.0 0.0 _rdoorrotation) false false))))

(fn ConstructionScript
  (|CallParentFunction))