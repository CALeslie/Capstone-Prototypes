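; Game mode for a local multiplayer minigame party game, cycling main menu, hub, minigame and score review until the final round crowns a winner.
; It spawns players, creates the UI and loads saved control settings.
; Each phase streams its level and delegates rules to an actor component, with Timelines driving fades and sequencing.
; A Tick-driven timer ends hub choices and hiding elimination rounds; only the hiding minigame is implemented.
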(event EventBeginPlay
  (CallFunction|GameSetup)
  (CallFunction|HandleGameSave)
  (switch Utilities|FlowControl|Switch|SwitchonEN_GameState (Variables|Default|GetCurrentGameState)
    (:NewEnumerator0
      (CallFunction|LoadMainMenu))
    (:NewEnumerator1
      (CallFunction|NewHubSession))
    (:NewEnumerator2
      (CallFunction|NewHidingGame :!label _label))
    (:NewEnumerator3
      (Development|PrintString "\"loading\" movement minigame")
      (goto _label))
    (:NewEnumerator4
      (Development|PrintString "\"loading\" manipulation minigame")
      (goto _label))))

(event EventTick
  (params (DeltaSeconds :type Float%20%28single-precision%29))
  (CallFunction|UpdateTimer DeltaSeconds)
  (CallFunction|TimerCheck))

(event EventHandleStartingNewPlayer
  (params (NewPlayer :type Player%20Controller%20Object%20Reference)))

(event EventPostLogin
  (params (NewPlayer :type Player%20Controller%20Object%20Reference))
  (Actor|DestroyActor NewPlayer))

(event Custom|CountdownFinished
  (bind _ac_hidingminigame (Variables|Default|GetAC_HidingMinigame))
  ;[1 1 1] Executes everytime the ingame timer reaches 0, handles eliminating players
  (Default|UpdateMinigameStatus (Variables|Default|GetAC_HidingMinigame) "NewEnumerator3")
  (bind _timeropacity (Timeline|EliminatePlayer PlayFromStart)
    (:Update
      (CallFunction|SetTimerOpacity _timeropacity) ; Fades out counter while playing elimination cutscene
    )
    (:ElimPlayerEvent
      (Default|EliminatePlayers _ac_hidingminigame))
    (:OpenDoorEvent
      (Default|OpenDoor _ac_hidingminigame))))

(event Custom|EliminationFinished
  (bind _ac_hidingminigame (Variables|Default|GetAC_HidingMinigame))
  (bind _ac_hidingminigame_2 (Variables|Default|GetAC_HidingMinigame))
  (bind _ac_hidingminigame_3 (Variables|Default|GetAC_HidingMinigame))
  ;[1 1 1] Executes after a round of eliminations is completed, checks if players are still left and if the game should be over or not, resets for another round of hiding if not
  (bind _result (Default|CheckPlayersLeft _ac_hidingminigame))
  (if _result
    (bind _timeropacity (Timeline|FinishElimination PlayFromStart)
      (:Update
        (if (not (Utilities|Enum|Equal(Enum) (Variables|/Game/Minigame/Blueprints/Minigames/Hiding/AC_HidingMinigame.AC_HidingMinigame_C|GetMinigameStatus (Variables|Default|GetAC_HidingMinigame)) "NewEnumerator2"))
          (CallFunction|SetTimerOpacity _timeropacity) ; Fades out counter while playing elimination cutscene
        ))
      (:Finished
        (Default|UpdateHidingSpots _ac_hidingminigame_3)
        (bind _result_2 (Default|CheckPlayersLeft _ac_hidingminigame_3))
        (if _result_2
          (Default|UpdateMinigameStatus (Variables|Default|GetAC_HidingMinigame) "NewEnumerator1")
          (else
            ;[1 1 1] This whole section handles wrapping up the end of the minigame
            (Default|UpdateMinigameStatus (Variables|Default|GetAC_HidingMinigame) "NewEnumerator2")
            (CallFunction|ToggleAllPlayersControl false)
            (for _array_element (Variables|Default|GetPlayers)
              (if (not (Variables|/Game/Minigame/Blueprints/BP_MinigameCharacter.BP_MinigameCharacter_C|GetCaught _array_element))
                (bind _output_get (Variables|Default|SetLastPlayer _array_element))
                (Utilities|Array|SetArrayElem (Variables|/Game/Minigame/Blueprints/Minigames/Hiding/AC_HidingMinigame.AC_HidingMinigame_C|GetPlayerRanks (Variables|Default|GetAC_HidingMinigame)) (Variables|/Game/Minigame/Blueprints/BP_MinigameCharacter.BP_MinigameCharacter_C|GetPlayerID _output_get) 1)))
            (Utilities|IsValid (Variables|Default|GetLastPlayer)
              (:Is%20Valid
                (CallFunction|SetCountdownText (Utilities|String|Append "Finished! P" (Utilities|String|ToString(Integer) (+ (Variables|/Game/Minigame/Blueprints/BP_MinigameCharacter.BP_MinigameCharacter_C|GetPlayerID (Variables|Default|GetLastPlayer)) 1)) " won"))
                (bind _fadealpha (Timeline|FinishedTimeline PlayFromStart)
                  (:Update
                    (CallFunction|SetCountdownOpacity _fadealpha))
                  (:Finished
                    (Utilities|FlowControl|Delay 3.0)
                    (bind _opacity (Timeline|BlackFadeIn PlayFromStart)
                      (:Update
                        (Default|SetBlackFadeOpacity (Variables|Default|GetMinigameUIRef) _opacity))
                      (:Finished
                        (CallFunction|SetPlayersVisibilities false)
                        (Class|GameplayStatics|UnloadStreamLevelbySoftObjectPtr "/Game/Minigame/Maps/HideNSneakLevel.HideNSneakLevel" true)
                        (CallFunction|LoadPostMinigame (Variables|/Game/Minigame/Blueprints/Minigames/Hiding/AC_HidingMinigame.AC_HidingMinigame_C|GetPlayerRanks (Variables|Default|GetAC_HidingMinigame))))))))
              (:Is%20Not%20Valid
                (CallFunction|SetCountdownText "Finished! No one won")
                (Timeline|FinishedTimeline PlayFromStart))))))
      (:CloseDoorEvent
        (Default|EventCloseDoor (Variables|/Game/Minigame/Blueprints/Minigames/Hiding/AC_HidingMinigame.AC_HidingMinigame_C|GetEnemyDoor _ac_hidingminigame_2))
        (Variables|Default|SetMinigameTimer (Variables|/Game/Minigame/Blueprints/Minigames/Hiding/AC_HidingMinigame.AC_HidingMinigame_C|GetTimeToHide _ac_hidingminigame_2))
        (CallFunction|SetTimerText)
        (Default|ReshowPlayers (Variables|Default|GetAC_HidingMinigame))))
    (else
      (Default|UpdateMinigameStatus _ac_hidingminigame "NewEnumerator2")
      (Timeline|FinishElimination PlayFromStart))))

(event Custom|NewHidingGame
  (Variables|Default|SetCurrentGameState "NewEnumerator2")
  (Class|GameplayStatics|LoadStreamLevelbySoftObjectPtr "/Game/Minigame/Maps/HideNSneakLevel.HideNSneakLevel" true true)
  ;[1 1 1] Sets up the AC component for the Hiding minigame when called
  (Default|MinigameSetup (Variables|Default|GetAC_HidingMinigame) self)
  (Default|SetCountdownText (Variables|Default|GetMinigameUIRef) "3")
  (Default|SetupEnemyandPlayers (Variables|Default|GetAC_HidingMinigame))
  (Utilities|FlowControl|Delay 0.25)
  (bind _opacity (Timeline|Timeline PlayFromStart)
    (:Update
      (Default|SetBlackFadeOpacity (Variables|Default|GetMinigameUIRef) _opacity))
    (:Finished
      ;[1 1 1] Executes at the beginning of the game to facilitate the countdown timer
      (bind _fadealpha (Timeline|CountdownTimeline PlayFromStart)
        (:Update
          (CallFunction|SetCountdownOpacity _fadealpha))
        (:ChangeText
          (CallFunction|TickCountdownStep))
        (:GivePlayerControl
          (CallFunction|ToggleAllPlayersControl true)
          (Default|UpdateMinigameStatus (Variables|Default|GetAC_HidingMinigame) "NewEnumerator1"))))))

(event Custom|NewHubSession
  (bind _ac_hub (Variables|Default|GetAC_Hub))
  (bind _currround (Variables|Default|GetCurrRound))
  (Math|Integer|IncrementInt _currround
    (:%20%20
      (if (<= _currround (Variables|Default|GetNumRounds))
        (Variables|Default|SetCurrentGameState "NewEnumerator1")
        (Class|GameplayStatics|LoadStreamLevelbySoftObjectPtr "/Game/Minigame/Maps/HubLevel.HubLevel" true true)
        (CallFunction|SetTimerOpacity 1.0)
        (Default|SetBlackFadeOpacity (Variables|Default|GetMinigameUIRef) 1.0)
        (Default|HubSetup _ac_hub self)
        (Default|SetUpPlayers _ac_hub)
        (Default|SetCountdownText (Variables|Default|GetMinigameUIRef))
        (Variables|Default|SetMinigameTimer (Variables|/Game/Minigame/Blueprints/Minigames/Hub/AC_HubMode.AC_HubMode_C|GetTimeToChoose (Variables|Default|GetAC_Hub)))
        (CallFunction|SetTimerText)
        (CallFunction|SetPlayersVisibilities true)
        (bind _fadeopacity (Timeline|HubFadeIn PlayFromStart)
          (:Update
            (Default|SetBlackFadeOpacity (Variables|Default|GetMinigameUIRef) _fadeopacity))
          (:Finished
            (CallFunction|ToggleAllPlayersControl true)))
        (else
          (CallFunction|EndOfGame))))))

(event Custom|ChoosingFinished
  (CallFunction|ToggleAllPlayersControl false)
  (Variables|/Game/Minigame/Blueprints/Minigames/Hub/AC_HubMode.AC_HubMode_C|SetHubStatus (Variables|Default|GetAC_Hub) "NewEnumerator1")
  (bind _timeropacity (Timeline|ChoosingFinishedAnim PlayFromStart)
    (:Update
      (CallFunction|SetTimerOpacity _timeropacity))
    (:Finished
      (Default|DetermineNextMinigame (Variables|Default|GetAC_Hub)))))

(event Custom|LoadNextMinigame
  (params (NextMinigameType :type EN_HubDoorType%20Enum :default "NewEnumerator0"))
  (Utilities|FlowControl|Delay 1.0)
  (bind _fadeopacity (Timeline|HubFadeOut PlayFromStart)
    (:Update
      (Default|SetBlackFadeOpacity (Variables|Default|GetMinigameUIRef) _fadeopacity))
    (:Finished
      (Class|GameplayStatics|UnloadStreamLevelbySoftObjectPtr "/Game/Minigame/Maps/HubLevel.HubLevel" true)
      (CallFunction|SetPlayersVisibilities false)
      (switch Utilities|FlowControl|Switch|SwitchonEN_HubDoorType NextMinigameType
        (:NewEnumerator0
          _)
        (:NewEnumerator1
          (Development|PrintString "Not Implemented Yet!" :!label _label))
        (:NewEnumerator2
          (goto _label)))
      (CallFunction|NewHidingGame))))

(event Custom|LoadMainMenu
  (bind _minigameuiref (Variables|Default|GetMinigameUIRef))
  (if (Variables|/Game/Minigame/Blueprints/Minigames/AC_MainMenu.AC_MainMenu_C|GetFirstLoad (Variables|Default|GetAC_MainMenu))
    (bind (_direction _splash1opacity _splash2opacity) (Timeline|ShowSplashScreens Play)
      (:Update
        (Default|SetSplashOpacity _minigameuiref 0 _splash1opacity)
        (Default|SetSplashOpacity _minigameuiref 1 _splash2opacity))
      (:Finished
        (Variables|/Game/Minigame/Blueprints/Minigames/AC_MainMenu.AC_MainMenu_C|SetFirstLoad (Variables|Default|GetAC_MainMenu) false)
        (Class|GameplayStatics|LoadStreamLevelbySoftObjectPtr "/Game/Minigame/Maps/MainMenuLevel.MainMenuLevel" true true :!label _label)
        (bind _blackfade (Timeline|FadeInMenu PlayFromStart)
          (:Update
            (Default|SetBlackFadeOpacity (Variables|Default|GetMinigameUIRef) _blackfade)
            (bind _result (Math|Float|NegateFloat _blackfade)
              (:%20%20
                (Default|SetMainMenuOpacity (Variables|Default|GetMinigameUIRef) (+ _result 1.0))))))))
    (else
      (goto _label))))

(event Custom|LoadHub
  (bind _blackfade (Timeline|FadeOutMenu PlayFromStart)
    (:Update
      (Default|SetBlackFadeOpacity (Variables|Default|GetMinigameUIRef) _blackfade))
    (:Finished
      (Default|SetMainMenuOpacity (Variables|Default|GetMinigameUIRef) 0.0)
      (Class|GameplayStatics|UnloadStreamLevelbySoftObjectPtr "/Game/Minigame/Maps/MainMenuLevel.MainMenuLevel" true)
      (CallFunction|NewHubSession))))

(event Custom|LoadPostMinigame
  (params (PrevGameRanks :type Array%20of%20Integers))
  (bind _ac_postminigame (Variables|Default|GetAC_PostMinigame))
  (Class|GameplayStatics|LoadStreamLevelbySoftObjectPtr "/Game/Minigame/Maps/ScoreReviewLevel.ScoreReviewLevel" true true)
  (Default|SetCountdownText (Variables|Default|GetMinigameUIRef))
  (Default|SetupPostMinigame (Variables|Default|GetAC_PostMinigame) self)
  (Default|DisplayNewScores _ac_postminigame PrevGameRanks)
  (Default|AwardPoints _ac_postminigame PrevGameRanks)
  (bind _opacity (Timeline|FadeInPostMinigame PlayFromStart)
    (:Update
      (Default|SetBlackFadeOpacity (Variables|Default|GetMinigameUIRef) _opacity))
    (:Finished
      (bind _opacity_2 (Timeline|FadeInScores PlayFromStart)
        (:Update
          (Variables|/Script/UMG.Widget|SetRenderOpacity (Variables|/Game/Minigame/Blueprints/WBP_MinigameUI.WBP_MinigameUI_C|GetPostMinigameCanvas (Variables|Default|GetMinigameUIRef)) _opacity_2))
        (:Finished
          (Utilities|FlowControl|Delay 5.0)
          (bind _opacity_3 (Timeline|FadeOutPostMinigame PlayFromStart)
            (:Update
              (Default|SetBlackFadeOpacity (Variables|Default|GetMinigameUIRef) _opacity_3)
              (bind _result (Math|Float|NegateFloat _opacity_3)
                (:%20%20
                  (Variables|/Script/UMG.Widget|SetRenderOpacity (Variables|/Game/Minigame/Blueprints/WBP_MinigameUI.WBP_MinigameUI_C|GetPostMinigameCanvas (Variables|Default|GetMinigameUIRef)) (+ _result 1.0)))))
            (:Finished
              (Class|GameplayStatics|UnloadStreamLevelbySoftObjectPtr "/Game/Minigame/Maps/ScoreReviewLevel.ScoreReviewLevel" true)
              (CallFunction|NewHubSession))))))))

(event Custom|EndOfGame
  (Variables|/Game/Minigame/Blueprints/AC_PostGame.AC_PostGame_C|SetGameModeRef (Variables|Default|GetAC_PostGame) self)
  (bind (_playernum _score) (Default|GetWinningPlayer (Variables|Default|GetAC_PostGame)))
  (CallFunction|SetCountdownText (Utilities|String|Append "P" (Utilities|String|ToString(Integer) _playernum) " is the winner, lowest score of " (Utilities|String|ToString(Integer) _score) " points!"))
  (Class|GameplayStatics|LoadStreamLevelbySoftObjectPtr "/Game/Minigame/Maps/HubLevel.HubLevel" true true)
  (bind _opacity (Timeline|FadeInWinText PlayFromStart)
    (:Update
      (CallFunction|SetCountdownOpacity _opacity)
      (bind _result (Math|Float|NegateFloat _opacity)
        (:%20%20
          (Default|SetBlackFadeOpacity (Variables|Default|GetMinigameUIRef) (+ _result 1.0)))))
    (:Finished
      (Utilities|FlowControl|Delay 5.0)
      (bind _opacity_2 (Timeline|FadeOutPostGame PlayFromStart)
        (:Update
          (Default|SetBlackFadeOpacity (Variables|Default|GetMinigameUIRef) _opacity_2))
        (:Finished
          (CallFunction|SetCountdownOpacity 0.0)
          (Class|GameplayStatics|UnloadStreamLevelbySoftObjectPtr "/Game/Minigame/Maps/HubLevel.HubLevel" true)
          (CallFunction|ResetGame))))))

(fn ConstructionScript)

(fn SpawnPlayers
  (bind _returnvalue (Game|GetPlayerController 0))
  (bind _returnvalue_2 (Game|GetPlayerController 0))
  (Variables|Default|SetDefaultPawnClass "/Game/Minigame/Blueprints/BP_MinigameCharacter.BP_MinigameCharacter_C")
  (Class|GameModeBase|RestartPlayer _returnvalue_2)
  (bind _asbp_minigame_character (Utilities|Casting|CastToBP_MinigameCharacter (Pawn|GetControlledPawn _returnvalue_2)))
  (CallFunction|SetPlayerMaterial (Variables|/Script/Engine.Character|GetMesh _asbp_minigame_character))
  (Default|TogglePlayerVisibility _asbp_minigame_character false)
  (Utilities|Array|AppendArray (Variables|Default|GetPlayers) (Utilities|Array|MakeArray _asbp_minigame_character))
  (for _index (range 0 3)
    ;[1 1 1] Creates player controller, if valid spawns character pawn at player start entity and then possesses pawn with that controller
    (bind _returnvalue_3 (Class|GameplayStatics|CreatePlayer -1))
    (if (Utilities|IsValid _returnvalue_3)
      (bind _returnvalue_4 (Game|SpawnActorfromClass "/Game/Minigame/Blueprints/BP_MinigameCharacter.BP_MinigameCharacter_C" (Math|Transform|MakeTransform "0, 0, 0" "0, 0, 0" "1.000000,1.000000,1.000000") "AlwaysSpawn" "MultiplyWithRoot" 0 0))
      (Pawn|Possess _returnvalue_3 _returnvalue_4)
      (Default|TogglePlayerVisibility _returnvalue_4 false)
      (Variables|/Game/Minigame/Blueprints/BP_MinigameCharacter.BP_MinigameCharacter_C|SetPlayerID _returnvalue_4 (+ _index 1))
      (Utilities|Array|AppendArray (Variables|Default|GetPlayers) (Utilities|Array|MakeArray _returnvalue_4))
      (CallFunction|SetPlayerMaterial (Variables|/Script/Engine.Character|GetMesh _returnvalue_4) (+ _index 1))))
  ;[1 1 1] Required to clean up default spawned controller
  (Class|GameModeBase|RestartPlayer _returnvalue)
  (bind _asbp_minigame_character_2 (Utilities|Casting|CastToBP_MinigameCharacter (Pawn|GetControlledPawn _returnvalue)))
  (Default|TogglePlayerVisibility _asbp_minigame_character_2 false)
  ;[1 1 1] Sends references of players back to movement controls UI to be modifiable on change
  (bind _foundwidgets (Widget|GetAllWidgetsOfClass "/Game/Minigame/Blueprints/WBP_MovementControls.WBP_MovementControls_C" false))
  (Default|RegisterPlayerActors (Utilities|Array|Get(acopy) _foundwidgets))
  (Variables|/Script/Engine.PlayerController|SetbShowMouseCursor (Game|GetPlayerController 0) true))

(fn TimerCheck
  (if (<= (Variables|Default|GetMinigameTimer) 0.1)
    (switch Utilities|FlowControl|Switch|SwitchonEN_GameState (Variables|Default|GetCurrentGameState)
      (:NewEnumerator1
        (if (Utilities|Enum|Equal(Enum) (Variables|/Game/Minigame/Blueprints/Minigames/Hub/AC_HubMode.AC_HubMode_C|GetHubStatus (Variables|Default|GetAC_Hub)) "NewEnumerator0")
          (CallFunction|ChoosingFinished)))
      (:NewEnumerator2
        (if (Utilities|Enum|Equal(Enum) (Variables|/Game/Minigame/Blueprints/Minigames/Hiding/AC_HidingMinigame.AC_HidingMinigame_C|GetMinigameStatus (Variables|Default|GetAC_HidingMinigame)) "NewEnumerator1")
          (CallFunction|CountdownFinished))))))

(fn UpdateTimer
  (params (Delta%20Time :type Float%20%28double-precision%29))
  ;[1 1 1] Updates minigame timer internally once per frame, updates UI element once per second
  (bind _minigamestatus (CallFunction|GetMinigameStatus))
  (if (Utilities|Enum|Equal(Enum) _minigamestatus "InProgress")
    (Variables|Default|SetMinigameTimer (- (Variables|Default|GetMinigameTimer) Delta%20Time))
    (bind _output_get (Variables|Default|SetMinigameUpdateTimer (+ (Variables|Default|GetMinigameUpdateTimer) Delta%20Time)))
    (if (>= _output_get 1.0)
      (Default|SetTimerText (Variables|Default|GetMinigameUIRef) (Utilities|Text|ToText(Integer) (Math|Float|Floor (Variables|Default|GetMinigameTimer))))
      (Math|Float|DecrementFloat (Variables|Default|GetMinigameUpdateTimer)))))

(fn ToggleAllPlayersControl
  (params (PlayerControl :type Boolean))
  (bind _outactors (Actor|GetAllActorsOfClass "/Game/Minigame/Blueprints/BP_MinigameCharacter.BP_MinigameCharacter_C"))
  (for _array_element _outactors
    (Variables|/Game/Minigame/Blueprints/BP_MinigameCharacter.BP_MinigameCharacter_C|SetControlEnabled _array_element PlayerControl)))

(fn CheckPlayersLeft
  (for _array_element (Variables|Default|GetPlayers)
    (if (not (Variables|/Game/Minigame/Blueprints/BP_MinigameCharacter.BP_MinigameCharacter_C|GetCaught _array_element))
      (Math|Integer|IncrementInt (LocalVariables|GetNumPlayersLeft))))
  (return (> (LocalVariables|GetNumPlayersLeft) 1)))

(fn SetTimerOpacity
  (params (NewOpacity :type Float%20%28double-precision%29))
  (Default|SetTimerOpacity (Variables|Default|GetMinigameUIRef) NewOpacity))

(fn SetCountdownOpacity
  (params (NewOpacity :type Float%20%28double-precision%29))
  (Default|SetCountdownOpacity (Variables|Default|GetMinigameUIRef) NewOpacity))

(fn TickCountdownStep
  (bind _minigameuiref (Variables|Default|GetMinigameUIRef))
  (switch int (Variables|Default|GetCountdownStep)
    (:0
      (Default|SetCountdownText _minigameuiref "2"))
    (:1
      (Default|SetCountdownText _minigameuiref "1"))
    (:2
      (Default|SetCountdownText _minigameuiref "Start!")))
  (Math|Integer|IncrementInt (Variables|Default|GetCountdownStep)))

(fn SetTimerText
  (Default|SetTimerText (Variables|Default|GetMinigameUIRef) (Utilities|Text|ToText(Integer) (Math|Float|Floor (Variables|Default|GetMinigameTimer)))))

(fn SetCountdownText
  (params (NewText :type String))
  (Default|SetCountdownText (Variables|Default|GetMinigameUIRef) (Utilities|Text|ToText(String) NewText)))

(fn HandleGameSave
  (bind _returnvalue (SaveGame|LoadGamefromSlot "GameSettings"))
  (Utilities|IsValid _returnvalue
    (:Is%20Valid
      (bind _asbp_game_save (Utilities|Casting|CastToBP_GameSave _returnvalue))
      (bind _output_get (Variables|Default|SetGameSaveRef _asbp_game_save))
      (Widget|GetAllWidgetsOfClass 0 true)
      (Default|LoadInstanceSettings (Variables|Default|GetMovementControlsRef) (Variables|/Game/Minigame/Blueprints/BP_GameSave.BP_GameSave_C|GetSavedPreset _output_get)))
    (:Is%20Not%20Valid
      (bind _returnvalue_2 (SaveGame|CreateSaveGameObject "/Game/Minigame/Blueprints/BP_GameSave.BP_GameSave_C"))
      (SaveGame|SaveGametoSlot _returnvalue_2 "GameSettings")))
  (return))

(fn GameSetup
  (bind _returnvalue (Game|GetPlayerController 0))
  (bind _returnvalue_2 (UserInterface|CreateWidget "/Game/Minigame/Blueprints/WBP_MinigameUI.WBP_MinigameUI_C" _returnvalue))
  (bind _output_get (Variables|Default|SetMinigameUIRef _returnvalue_2))
  (UserInterface|Viewport|AddtoViewport _output_get 0)
  (Default|SetGamemodeRef _output_get self)
  (bind _returnvalue_3 (UserInterface|CreateWidget "/Game/Minigame/Blueprints/WBP_MovementControls.WBP_MovementControls_C" _returnvalue))
  (bind _output_get_2 (Variables|Default|SetMovementControlsRef _returnvalue_3))
  (UserInterface|Viewport|AddtoViewport _output_get_2 0)
  (CallFunction|SpawnPlayers))

(fn GetMinigameStatus
  (switch Utilities|FlowControl|Switch|SwitchonEN_GameState (Variables|Default|GetCurrentGameState)
    (:NewEnumerator1
      (return (Utilities|String|EnumtoString (Variables|/Game/Minigame/Blueprints/Minigames/Hub/AC_HubMode.AC_HubMode_C|GetHubStatus (Variables|Default|GetAC_Hub)))))
    (:NewEnumerator2
      (return (Utilities|String|EnumtoString (Variables|/Game/Minigame/Blueprints/Minigames/Hiding/AC_HidingMinigame.AC_HidingMinigame_C|GetMinigameStatus (Variables|Default|GetAC_HidingMinigame)))))))

(fn SetPlayerMaterial
  (params (PlayerMesh :type Skeletal%20Mesh%20Component%20Object%20Reference) (Index :type Integer))
  (switch int Index
    (:0
      (Rendering|Material|SetMaterial PlayerMesh 0 "/Game/Characters/Mannequins/Materials/Instances/Quinn/MI_Player1Mat_01.MI_Player1Mat_01")
      (Rendering|Material|SetMaterial PlayerMesh 1 "/Game/Characters/Mannequins/Materials/Instances/Quinn/MI_Player1Mat_02.MI_Player1Mat_02"))
    (:1
      (Rendering|Material|SetMaterial PlayerMesh 0 "/Game/Characters/Mannequins/Materials/Instances/Quinn/MI_Player2Mat_01.MI_Player2Mat_01")
      (Rendering|Material|SetMaterial PlayerMesh 1 "/Game/Characters/Mannequins/Materials/Instances/Quinn/MI_Player2Mat_02.MI_Player2Mat_02"))
    (:2
      (Rendering|Material|SetMaterial PlayerMesh 0 "/Game/Characters/Mannequins/Materials/Instances/Quinn/MI_Player3Mat_01.MI_Player3Mat_01")
      (Rendering|Material|SetMaterial PlayerMesh 1 "/Game/Characters/Mannequins/Materials/Instances/Quinn/MI_Player3Mat_02.MI_Player3Mat_02"))
    (:3
      (Rendering|Material|SetMaterial PlayerMesh 0 "/Game/Characters/Mannequins/Materials/Instances/Quinn/MI_Player4Mat_01.MI_Player4Mat_01")
      (Rendering|Material|SetMaterial PlayerMesh 1 "/Game/Characters/Mannequins/Materials/Instances/Quinn/MI_Player4Mat_02.MI_Player4Mat_02"))))

(fn ResetGame
  (for _index (range 0 3)
    (Utilities|Array|SetArrayElem (Variables|Default|GetPlayerScores) _index 0)
    (Variables|Default|SetCurrRound 0)
    (CallFunction|LoadMainMenu)))

(fn SetPlayersVisibilities
  (params (Visible :type Boolean))
  (for _array_element (Variables|Default|GetPlayers)
    (Default|TogglePlayerVisibility _array_element Visible)))